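; BP_CoreTestCharacter is a player character in the HUD demo that can move, look around and interact.
; On BeginPlay it adds the IMC_CoreTestPlayer Enhanced Input mapping context to its player controller.
; Movement follows the camera's forward and right vectors without flattening them, and camera input drives controller yaw and pitch.
; The interact action calls Interact on its Interactor, which holds the interaction logic outside this graph.
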(event `self.ReceiveBeginPlay`
  (bind _asplayer_controller (cast `PlayerController` (`self.GetController`)))
  (`EnhancedInputSubsystemInterface.AddMappingContext` (pcsubsystem `EnhancedInputLocalPlayerSubsystem` _asplayer_controller) "/Game/HUDDemo/IMC_CoreTestPlayer.IMC_CoreTestPlayer" 0 (struct)))

(event `EnhancedInput|/Game/HUDDemo/IA_Interact`
  (params (ActionValue :type Boolean) (ElapsedSeconds :type "Float (double-precision)") (TriggeredSeconds :type "Float (double-precision)") (InputAction :type "InputAction Object Reference" :default "/Game/HUDDemo/IA_Interact.IA_Interact"))
  (:`Triggered`
    (`InteractorComponent.Interact` (`self.Interactor`))))

(event `EnhancedInput|/Game/HUDDemo/IA_Move`
  (params (ActionValue :type "Vector2D Structure") (ElapsedSeconds :type "Float (double-precision)") (TriggeredSeconds :type "Float (double-precision)") (InputAction :type "InputAction Object Reference" :default "/Game/HUDDemo/IA_Move.IA_Move"))
  (bind _camera (`self.Camera`))
  (:`Triggered`
    (`self.AddMovementInput` (`SceneComponent.GetForwardVector` _camera) ActionValue_Y)
    (`self.AddMovementInput` (`SceneComponent.GetRightVector` _camera) ActionValue_X)))

(event `EnhancedInput|/Game/HUDDemo/IA_Camera`
  (params (ActionValue :type "Vector2D Structure") (ElapsedSeconds :type "Float (double-precision)") (TriggeredSeconds :type "Float (double-precision)") (InputAction :type "InputAction Object Reference" :default "/Game/HUDDemo/IA_Camera.IA_Camera"))
  (:`Triggered`
    (`self.AddControllerYawInput` ActionValue_X)
    (`self.AddControllerPitchInput` ActionValue_Y)))

(fn `UserConstructionScript`)