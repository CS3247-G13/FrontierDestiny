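; BP_QuestMarkerActor is a quest marker that hovers above the current quest target and hides when the player comes within HideDistance.
; It binds to the quest subsystem's update event on BeginPlay to cache the quest and target and set initial visibility.
; Tick follows the target and toggles the marker by player distance.
; Inside the hide range, a hardcoded proximity check calls CompleteObjective for Quest_One only, on every qualifying frame.
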(event `self.ReceiveTick`
  (params (DeltaSeconds :type "Float (single-precision)"))
  (bind _questmarker (`self.QuestMarker`))
  (if (`KismetSystemLibrary.IsValid` (stale `EventQuestUpdate` _output_get_2))
    (bind _returnvalue (`self.K2_GetActorLocation` (stale `EventQuestUpdate` _output_get_2)))
    (`self.K2_SetActorLocation` (+ _returnvalue (0.0 0.0 150.0)))
    (bind _returnvalue_2 (`KismetMathLibrary.Vector_Distance` (`self.K2_GetActorLocation` (`GameplayStatics.GetPlayerCharacter` 0)) _returnvalue))
    (if (< _returnvalue_2 (`self.HideDistance`))
      (`SceneComponent.SetVisibility` _questmarker false false)
      (if (< _returnvalue_2 500.0)
        (if (== (`.QuestID` (break `QuestData` (`self.Quest`))) "Quest_One")
          (`QuestSubsystem.CompleteObjective` (subsystem `QuestSubsystem`))))
      (else
        (`SceneComponent.SetVisibility` _questmarker true false)))))

(event `self.ReceiveBeginPlay`
  (add `QuestSubsystem.OnQuestUpdated` (subsystem `QuestSubsystem`) (delegate `EventQuestUpdate`)))

(event `EventQuestUpdate`
  (params (Quest :type "QuestData Structure (by ref)"))
  (bind _questmarker (`self.QuestMarker`))
  (bind _output_get (set `self.Quest` Quest))
  (bind _output_get_2 (set `self.Quest Target` (`.Target` (break `QuestData` _output_get))))
  (if (`KismetSystemLibrary.IsValid` _output_get_2)
    (`SceneComponent.SetVisibility` _questmarker true false)
    (else
      (`SceneComponent.SetVisibility` _questmarker false false))))

(fn `UserConstructionScript`)