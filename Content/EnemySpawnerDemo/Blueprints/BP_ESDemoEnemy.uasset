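; Demo enemy for the enemy spawner demo that walks to the core actor, damages it on arrival and destroys itself.
; A looping timer issues the AI move order toward the first core actor found at start.
; Tick updates an overhead health bar from the stat component's HP and turns it toward the camera.
; On taking damage, it destroys itself if HP is depleted.
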(event `Start`
  (bind _outactors (`GameplayStatics.GetAllActorsOfClass` "/Game/FrontierDestiny/05_Core/BP_CoreActor.BP_CoreActor_C"))
  (set `self.Target` (`|GetArrayItem` _outactors))
  (bind _outactors_2 (`GameplayStatics.GetAllActorsOfClass` "/Game/FrontierDestiny/01_Player/Blueprints/BP_Player.BP_Player_C"))
  (set `self.Player` (`|GetArrayItem` _outactors_2))
  (`KismetSystemLibrary.K2_SetTimer` null "MoveNPC" 5.0 true)
  (`KismetSystemLibrary.PrintString` "Walking"))

(event `self.ReceiveTick`
  (params (DeltaSeconds :type "Float (single-precision)"))
  (bind _health_bar_widget (`self.Health Bar Widget`))
  (bind _statcomponent (`self.StatComponent`))
  (bind _aswb_health_bar (cast `/Game/EnemySpawnerDemo/Blueprints/WB_HealthBar` (`WidgetComponent.GetWidget` (`self.Health Bar Widget`))))
  (`ProgressBar.SetPercent` (`/Game/EnemySpawnerDemo/Blueprints/WB_HealthBar.HealthBar` _aswb_health_bar) (/ (`StatComponent.GetStat` _statcomponent "HP") (`StatComponent.GetBaseStat` _statcomponent "HP")))
  (`SceneComponent.K2_SetWorldRotation` _health_bar_widget (`KismetMathLibrary.FindLookAtRotation` (`SceneComponent.K2_GetComponentLocation` _health_bar_widget) (`SceneComponent.K2_GetComponentLocation` (`Actor.RootComponent` (`GameplayStatics.GetPlayerCameraManager` 0)))) false false))

(event `self.ReceiveAnyDamage`
  (params (Damage :type "Float (single-precision)") (DamageType :type "DamageType Object Reference") (InstigatedBy :type "Controller Object Reference") (DamageCauser :type "Actor Object Reference"))
  (if (<= (`StatComponent.GetStat` (`self.StatComponent`) "HP") 0.0)
    (`self.K2_DestroyActor`)))

(event `MoveNPC`
  (bind _target (`self.Target`))
  (`|AIMoveTo` self (0.0 0.0 0.0) _target 10.0
    (:`OnSuccess`
      (`KismetSystemLibrary.PrintString` "Hello")
      (`GameplayStatics.ApplyDamage` _target 5.0)
      (`self.K2_DestroyActor`))))

(fn `UserConstructionScript`)