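; BP_ESDemoEnemySpawner is a demo spawner actor that releases a wave of BP_ESDemoEnemy on BeginPlay.
; A looping timer spawns each enemy at a random reachable navmesh point around the spawner and calls its Start.
; Each enemy randomly stays unmodified or gets a Fast or Slow modifier through its StatComponent, and the timer clears once the wave's spawn limit is reached.
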(event `self.ReceiveBeginPlay`
  (`self.Wave 1`))

(event `Wave 1`
  (bind _returnvalue (`KismetSystemLibrary.K2_SetTimerDelegate` (delegate `SpawnEnemy`) 2.0 true))
  (set `self.CurrentTimer` _returnvalue)
  (set `self.MaxSpawnCount` 10.0)
  (set `self.CurrentSpawnCount` 0.0))

(event `SpawnEnemy`
  (`/Engine/EditorBlueprintResources/StandardMacros.IncrementFloat` (`self.CurrentSpawnCount`)
    (:`  `
      (bind _returnvalue (`|SpawnActorFromClass` "/Game/EnemySpawnerDemo/Blueprints/BP_ESDemoEnemy.BP_ESDemoEnemy_C" (`KismetMathLibrary.Conv_VectorToTransform` (`NavigationSystemV1.K2_GetRandomReachablePointInRadius` (`self.K2_GetActorLocation`) 300.0 null null)) "AdjustIfPossibleButAlwaysSpawn" "MultiplyWithRoot" null null))
      (`/Game/EnemySpawnerDemo/Blueprints/BP_ESDemoEnemy.Start` _returnvalue)
      (switch `int` (`KismetMathLibrary.RandomInteger` 3)
        (:`0`
          _)
        (:`1`
          (bind _statcomponent (`BaseEnemyCharacter.StatComponent` _returnvalue))
          (`StatComponent.ApplyModifier` _statcomponent "/Game/EnemySpawnerDemo/Blueprints/Fast.Fast"))
        (:`2`
          (`StatComponent.ApplyModifier` _statcomponent "/Game/EnemySpawnerDemo/Blueprints/Slow.Slow")))
      (if (<= (`self.MaxSpawnCount`) (`self.CurrentSpawnCount`))
        (`KismetSystemLibrary.K2_ClearAndInvalidateTimerHandle` (`self.CurrentTimer`))))))

(fn `UserConstructionScript`)