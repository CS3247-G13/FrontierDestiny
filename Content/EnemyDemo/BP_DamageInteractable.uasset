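; BP_DamageInteractable is a demo actor the player can pick up and carry, which damages actors it touches.
; Pickup and Drop toggle a Grab flag, and while it is set Tick moves the actor to a fixed distance along the player camera's forward vector, without sweep.
; The Cube component's begin overlap applies damage to the overlapping actor, with itself as the damage causer.
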(event `Pickup`
  (set `self.grab` true))

(event `Drop`
  (set `self.grab` false))

(event `self.ReceiveTick`
  (params (DeltaSeconds :type "Float (single-precision)"))
  (bind _playercameramanager (`PlayerController.PlayerCameraManager` (`GameplayStatics.GetPlayerController` 0)))
  (if (`self.grab`)
    (`self.K2_SetActorLocation` (+ (* (`KismetMathLibrary.GetForwardVector` (`PlayerCameraManager.GetCameraRotation` _playercameramanager)) 700.0) (`PlayerCameraManager.GetCameraLocation` _playercameramanager)))))

(event `self.Cube.OnComponentBeginOverlap`
  (params (OverlappedComponent :type "PrimitiveComponent Object Reference") (OtherActor :type "Actor Object Reference") (OtherComp :type "PrimitiveComponent Object Reference") (OtherBodyIndex :type Integer) (bFromSweep :type Boolean) (SweepResult :type "HitResult Structure (by ref)"))
  (`GameplayStatics.ApplyDamage` OtherActor 10.0 null self))

(fn `UserConstructionScript`)