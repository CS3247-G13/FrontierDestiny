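; BP_TeslaChain is a tesla chain effect actor that fires a particle beam from itself at a target.
; Each tick it calls Attack while Target is valid, and otherwise calls SelectTarget to acquire one.
; Attack spawns a new Niagara system on every call, setting its Origin and Target vector parameters to the two actors' locations.
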(event `self.ReceiveTick`
  (params (DeltaSeconds :type "Float (single-precision)"))
  (`/Engine/EditorBlueprintResources/StandardMacros.IsValid` (`self.Target`)
    (:`Is Valid`
      (`self.Attack`))
    (:`Is Not Valid`
      (`self.SelectTarget`))))

(fn `Attack`
  (bind _returnvalue (`NiagaraFunctionLibrary.SpawnSystemAtLocation` null))
  (`NiagaraComponent.SetVariableVec3` _returnvalue "Origin" (`self.K2_GetActorLocation`))
  (`NiagaraComponent.SetVariableVec3` _returnvalue "Target" (`self.K2_GetActorLocation` (`self.Target`))))

(fn `UserConstructionScript`)