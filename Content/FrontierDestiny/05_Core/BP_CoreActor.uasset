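; Core actor that takes damage and visually shows whether it is activated.
; Its sphere starts with a deactivated material and switches when OnCoreActivated fires, while any incoming damage is forwarded to ApplyDamage.
; Each tick box-traces at the cylinder for instanced static mesh hits, but the logic to destroy that enemy instance through EnemyManagerSubsystem and damage the core is disconnected.
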(event `self.ReceiveAnyDamage`
  (params (Damage :type "Float (single-precision)") (DamageType :type "DamageType Object Reference") (InstigatedBy :type "Controller Object Reference") (DamageCauser :type "Actor Object Reference"))
  (`self.ApplyDamage` Damage))

(event `self.ReceiveBeginPlay`
  (add `self.OnCoreActivated` (delegate `OnCoreActivated_Event`))
  (`PrimitiveComponent.SetMaterial` (`self.Sphere`) 0 (`self.Deactivated Material`)))

(event `OnCoreActivated_Event` :!signature `self.OnCoreActivated`
  (params (CoreActor :type "CoreActor Object Reference"))
  (`PrimitiveComponent.SetMaterial` (`self.Sphere`) 0 (`self.Activated Material`)))

(event `self.ReceiveTick`
  (params (DeltaSeconds :type "Float (single-precision)"))
  (bind _returnvalue (`SceneComponent.K2_GetComponentLocation` (`self.Cylinder`)))
  (bind _outhit (`KismetSystemLibrary.BoxTraceSingle` _returnvalue _returnvalue (30.0 30.0 30.0) (struct) "TraceTypeQuery1"))
  (bind _asinstanced_static_mesh_component (cast `InstancedStaticMeshComponent` (`.HitComponent` (`GameplayStatics.BreakHitResult` _outhit)))))

(fn `UserConstructionScript`)