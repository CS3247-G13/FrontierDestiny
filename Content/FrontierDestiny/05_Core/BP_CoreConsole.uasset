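; BP_CoreConsole is an interactable console that activates a linked Core and unlocks upgrade blueprints.
; It starts with a disabled screen material; on interaction it activates the Core, lights the screen and deactivates its Interactable component.
; It then unlocks each entry in UpgradeBlueprints through the UpgradeManagerSubsystem and completes the QuestSubsystem objective if the current quest targets this console.
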(event `self.ReceiveBeginPlay`
  (`PrimitiveComponent.SetMaterial` (`self.Cube`) 2 (`self.Disabled Material`))
  (`KismetSystemLibrary.Delay` 0.2))

(event `self.Interactable.OnInteracted`
  (params (Interactor :type "Actor Object Reference"))
  (bind _returnvalue (subsystem `QuestSubsystem`))
  (bind (_currentquest_questid _currentquest_messages _currentquest_prompt _currentquest_currentmessageindex _currentquest_targettag) (break `QuestData` (`QuestSubsystem.CurrentQuest` _returnvalue)))
  (`CoreActor.ActivateCore` (`self.Core`))
  (`PrimitiveComponent.SetMaterial` (`self.Cube`) 2 (`self.Screen Material`))
  (`InteractableComponent.DeactivateInteractable` (`self.Interactable`))
  (for _array_element (`self.Upgrade Blueprints`)
    (`UpgradeManagerSubsystem.UnlockBlueprint` (subsystem `UpgradeManagerSubsystem`) _array_element))
  (if (== _currentquest_targettag "Core_Console")
    (`QuestSubsystem.CompleteObjective` _returnvalue)))

(fn `UserConstructionScript`)