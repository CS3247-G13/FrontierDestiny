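; BP_InvisibleWall is a quest-gated boundary volume that keeps the player from leaving its Box during a span of quests.
; Tick polls the QuestSubsystem, setting the Box to overlap on a custom trace channel at StartQuestID and ignore it at EndQuestID.
; Tick also records the player pawn's location every frame, and any end overlap on the Box moves the pawn back to that location.
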(event `self.ReceiveTick`
  (params (DeltaSeconds :type "Float (single-precision)"))
  (bind _box (`self.Box`))
  (bind _currentquest_questid (break `QuestData` (`QuestSubsystem.CurrentQuest` (subsystem `QuestSubsystem`))))
  (if (== _currentquest_questid (`self.StartQuestID`))
    (`PrimitiveComponent.SetCollisionResponseToChannel` _box "ECC_GameTraceChannel5" "ECR_Overlap")
    (elif (== (`self.EndQuestID`) _currentquest_questid)
      (`PrimitiveComponent.SetCollisionResponseToChannel` _box "ECC_GameTraceChannel5" "ECR_Ignore")))
  (set `self.LastValidLocation` (`self.K2_GetActorLocation` (`GameplayStatics.GetPlayerPawn` 0))))

(event `self.Box.OnComponentEndOverlap`
  (params (OverlappedComponent :type "PrimitiveComponent Object Reference") (OtherActor :type "Actor Object Reference") (OtherComp :type "PrimitiveComponent Object Reference") (OtherBodyIndex :type Integer))
  (bind _returnvalue (`GameplayStatics.GetPlayerPawn` 0))
  (if (`KismetSystemLibrary.IsValid` _returnvalue)
    (`self.K2_SetActorLocation` _returnvalue (`self.LastValidLocation`) false false)))

(fn `UserConstructionScript`)