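; Interactable blueprint cache chest that unlocks and purchases the upgrade matching its UpgradeID when opened.
; It registers with the cache manager and plays an ambient cue on BeginPlay, listening to its Interactable component.
; Interaction plays the open animation and sound, shows floating unlock text, calls the upgrade manager, deregisters the cache, stops the ambience and starts the "Blueprint" quest.
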(event `self.ReceiveBeginPlay`
  (add `InteractableComponent.OnInteracted` (`self.Interactable`) (delegate `OnInteracted_Event`))
  (`CacheManagerSubsystem.RegisterCache` (subsystem `CacheManagerSubsystem`) self)
  (`AudioComponent.Play` (`self.Cue_Cache_Ambient`) 0.0))

(event `self.ReceiveEndPlay`
  (params (EndPlayReason :type "EEndPlayReason Enum" :default "Destroyed"))
  (bind _interactable (`self.Interactable`))
  (`/Engine/EditorBlueprintResources/StandardMacros.IsValid` _interactable
    (:`Is Valid`
      (clear `InteractableComponent.OnInteracted` _interactable))))

(event `OnInteracted_Event`
  (params (Interactor :type "Actor Object Reference"))
  (bind _returnvalue (subsystem `UpgradeManagerSubsystem`))
  (bind _upgradeid (`self.UpgradeID`))
  (`/Engine/EditorBlueprintResources/StandardMacros.IsValid` (`self.Interactable`)
    (:`Is Valid`
      (`SkeletalMeshComponent.PlayAnimation` (`self.SkeletalMesh`) "/Game/FrontierDestiny/06_Interactable/chest/sci-fi_futuristic_container/SkeletalMeshes/CacheMesh_Anim.CacheMesh_Anim" false)
      (`|SpawnActorFromClass` "/Game/FrontierDestiny/99_Testing/BP_DisappearingText.BP_DisappearingText_C" (`KismetMathLibrary.MakeTransform` (+ (.location (`self.GetTransform`)) (0.0 0.0 50.0)) (.rotation (`self.GetTransform`)) (.scale (`self.GetTransform`))) "Undefined" "MultiplyWithRoot" null (`KismetTextLibrary.Conv_StringToText` (`KismetStringLibrary.Concat_StrStr` "Unlock " (`.Name` (break `UpgradeData` (`UpgradeManagerSubsystem.GetUpgradeData` _returnvalue (`self.UpgradeID`)))) " blueprint")) null)
      (`UpgradeManagerSubsystem.UnlockBlueprint` _returnvalue _upgradeid)
      (`UpgradeManagerSubsystem.PurchaseUpgrade` _returnvalue _upgradeid)
      (`CacheManagerSubsystem.DeregisterCache` (subsystem `CacheManagerSubsystem`) self)
      (`GameplayStatics.PlaySoundAtLocation` "/Game/FrontierDestiny/06_Interactable/chest/Sounds/Cache_Open.Cache_Open" (`self.K2_GetActorLocation` self) (struct) 1.0 1.0 0.0 null null null null)
      (`AudioComponent.Stop` (`self.Cue_Cache_Ambient`))
      (`QuestSubsystem.StartQuest` (subsystem `QuestSubsystem`) "Blueprint"))))

(fn `UserConstructionScript`)