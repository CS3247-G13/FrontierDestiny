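; BP_Mimic is an interactable trap chest that spawns an enemy when used.
; On BeginPlay it binds to its Interactable component's OnInteracted event, and it clears the bindings on EndPlay.
; Interaction plays the chest animation, spawns "Surprise" disappearing text above it, then after a short delay force-spawns a BP_ESDemoEnemy overhead and calls Start on it.
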(event `self.ReceiveBeginPlay`
  (add `InteractableComponent.OnInteracted` (`self.Interactable`) (delegate `OnInteracted_Event`)))

(event `self.ReceiveEndPlay`
  (params (EndPlayReason :type "EEndPlayReason Enum" :default "Destroyed"))
  (bind _interactable (`self.Interactable`))
  (`/Engine/EditorBlueprintResources/StandardMacros.IsValid` _interactable
    (:`Is Valid`
      (clear `InteractableComponent.OnInteracted` _interactable))))

(event `OnInteracted_Event`
  (params (Interactor :type "Actor Object Reference"))
  (`/Engine/EditorBlueprintResources/StandardMacros.IsValid` (`self.Interactable`)
    (:`Is Valid`
      (`SkeletalMeshComponent.PlayAnimation` (`self.SkeletalMesh`) "/Game/FrontierDestiny/06_Interactable/chest/SkeletalMeshes/chest_Anim.chest_Anim" false)
      (`|SpawnActorFromClass` "/Game/FrontierDestiny/99_Testing/BP_DisappearingText.BP_DisappearingText_C" (`KismetMathLibrary.MakeTransform` (+ (.location (`self.GetTransform`)) (0.0 0.0 50.0)) (.rotation (`self.GetTransform`)) (.scale (`self.GetTransform`))) "Undefined" "MultiplyWithRoot" null "Surprise" null)
      (`KismetSystemLibrary.Delay` 1.0)
      (bind _returnvalue (`|SpawnActorFromClass` "/Game/FrontierDestiny/02_Enemy/BP_ESDemoEnemy.BP_ESDemoEnemy_C" (`KismetMathLibrary.MakeTransform` (+ (.location (`self.GetTransform`)) (0.0 0.0 100.0)) (.rotation (`self.GetTransform`))) "AlwaysSpawn" "MultiplyWithRoot" null null))
      (`/Game/FrontierDestiny/02_Enemy/BP_ESDemoEnemy.Start` _returnvalue))))

(fn `UserConstructionScript`)