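; BP_Money is an interactable chest that grants the player resources.
; It binds to its Interactable component's OnInteracted event on BeginPlay and unbinds on EndPlay.
; Interacting plays the chest animation, spawns floating BP_DisappearingText above it and adds Cryxite, Nullsteel and Gravstone through the economy subsystem.
; The popup text is hardcoded independently of the granted amounts, and nothing in the graph blocks repeat interactions.
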(event `self.ReceiveBeginPlay`
  (add `InteractableComponent.OnInteracted` (`self.Interactable`) (delegate `OnInteracted_Event`)))

(event `self.ReceiveEndPlay`
  (params (EndPlayReason :type "EEndPlayReason Enum" :default "Destroyed"))
  (bind _interactable (`self.Interactable`))
  (`/Engine/EditorBlueprintResources/StandardMacros.IsValid` _interactable
    (:`Is Valid`
      (clear `InteractableComponent.OnInteracted` _interactable))))

(event `OnInteracted_Event`
  (params (Interactor :type "Actor Object Reference"))
  (`/Engine/EditorBlueprintResources/StandardMacros.IsValid` (`self.Interactable`)
    (:`Is Valid`
      (`SkeletalMeshComponent.PlayAnimation` (`self.SkeletalMesh`) "/Game/FrontierDestiny/06_Interactable/chest/SkeletalMeshes/chest_Anim.chest_Anim" false)
      (`|SpawnActorFromClass` "/Game/FrontierDestiny/99_Testing/BP_DisappearingText.BP_DisappearingText_C" (`KismetMathLibrary.MakeTransform` (+ (.location (`self.GetTransform`)) (0.0 0.0 50.0)) (.rotation (`self.GetTransform`)) (.scale (`self.GetTransform`))) "Undefined" "MultiplyWithRoot" null "+500 cryxite" null)
      (`EconomySubsystem.AddFunds` (subsystem `EconomySubsystem`) (make `ResourceAmount` (`self.Cryxite`) (`self.NullSteel`) (`self.GravStone`))))))

(fn `UserConstructionScript`)