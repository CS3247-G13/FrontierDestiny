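; Demo enemy that rushes the core to deal damage and then hits itself for its current HP, or attacks the player when no active core exists.
; Start plays a random laugh, caches the player, polls for a CoreActor until found, and loops MoveNPC on a timer to re-issue AIMoveTo.
; Tick feeds StatComponent HP into a camera-facing health bar.
; AnyDamage spawns randomly offset floating damage text facing the player.
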(event `MoveNPC`
  (bind _target (`self.Target`))
  (bind _statcomponent (`self.StatComponent`))
  (bind _returnvalue (`StatComponent.GetStat` _statcomponent "Damage"))
  (if (and (`KismetSystemLibrary.IsValid` _target) (`CoreActor.bIsCoreActive` _target))
    ;[0.3229 0.00113 0.001674 0] If the core is valid, path to it and deal 5 damage
    (`|AIMoveTo` self (0.0 0.0 0.0) (`self.Target`) 10.0
      (:`OnSuccess`
        (`GameplayStatics.ApplyDamage` (`self.Target`) _returnvalue)
        (`GameplayStatics.ApplyDamage` self (`StatComponent.GetStat` _statcomponent "HP"))
        (`KismetSystemLibrary.PrintString` "Hello")))
    (else
      ;[0 0.03463 0.3229 0] Else, go hit the player instead
      (`|AIMoveTo` self (0.0 0.0 0.0) (`self.Player`) 10.0
        (:`OnSuccess`
          (`GameplayStatics.ApplyDamage` (`self.Player`) _returnvalue))))))

(event `Start`
  (`|ExecutionSequence`
    (:`then_0`
      ;[0 0 0 0.5] Play a random sound when the enemy is spawned
      (`GameplayStatics.PlaySoundAtLocation` (select `bool` (`KismetMathLibrary.RandomBool`) :`false` "/Game/FrontierDestiny/02_Enemy/Audio/Female_hearty_cackling_laughter_M.Female_hearty_cackling_laughter_M" :`true` "/Game/FrontierDestiny/02_Enemy/Audio/Joyful_male_laughter_01_M.Joyful_male_laughter_01_M" :!type "SoundBase Object Reference") (`self.K2_GetActorLocation`) (struct) 1.0 1.0 0.0 null null null null))
    (:`then_1`
      (bind _returnvalue (`KismetSystemLibrary.K2_SetTimerDelegate` (delegate `Check for core`) 2.0 true)))
    (:`then_2`
      ;[0 0 0 0.5] Set the target to be the grid and get a reference to the player
      (bind _outactors (`GameplayStatics.GetAllActorsOfClass` "/Script/FrontierDestiny.CoreActor" :!label _label))
      (bind _output_get (set `self.Target` (`|GetArrayItem` _outactors)))
      (`/Engine/EditorBlueprintResources/StandardMacros.IsValid` _output_get
        (:`Is Valid`
          (`KismetSystemLibrary.K2_ClearAndInvalidateTimerHandle` _returnvalue))))
    (:`then_3`
      ;[0 0 0] Initialize the movement logic
      (`self.MoveNPC`)
      (`KismetSystemLibrary.K2_SetTimer` null "MoveNPC" 0.2 true))
    (:`then_4`
      (bind _outactors_2 (`GameplayStatics.GetAllActorsOfClass` "/Game/FrontierDestiny/01_Player/Blueprints/BP_Player.BP_Player_C"))
      (set `self.Player` (`|GetArrayItem` _outactors_2)))))

(event `Check for core`
  ;[0 0 0 0.5] Set the target to be the grid and get a reference to the player
  (goto _label))

(event `self.ReceiveTick`
  (params (DeltaSeconds :type "Float (single-precision)"))
  (bind _health_bar_widget (`self.Health Bar Widget`))
  (bind _statcomponent (`self.StatComponent`))
  ;[0 0 0] Update the healthbar's percentage and rotation to face the player
  (bind _aswb_health_bar (cast `/Game/FrontierDestiny/02_Enemy/WB_HealthBar` (`WidgetComponent.GetWidget` (`self.Health Bar Widget`))))
  (`ProgressBar.SetPercent` (`/Game/FrontierDestiny/02_Enemy/WB_HealthBar.HealthBar` _aswb_health_bar) (/ (`StatComponent.GetStat` _statcomponent "HP") (`StatComponent.GetBaseStat` _statcomponent "HP")))
  (`SceneComponent.K2_SetWorldRotation` _health_bar_widget (`KismetMathLibrary.FindLookAtRotation` (`SceneComponent.K2_GetComponentLocation` _health_bar_widget) (`SceneComponent.K2_GetComponentLocation` (`Actor.RootComponent` (`GameplayStatics.GetPlayerCameraManager` 0)))) false false))

(event `self.ReceiveAnyDamage`
  (params (Damage :type "Float (single-precision)") (DamageType :type "DamageType Object Reference") (InstigatedBy :type "Controller Object Reference") (DamageCauser :type "Actor Object Reference"))
  (bind _location (.location (`self.GetTransform`)))
  (bind _returnvalue (`KismetMathLibrary.MakeRotFromX` (`KismetMathLibrary.GetDirectionUnitVector` _location (`self.K2_GetActorLocation` (`GameplayStatics.GetPlayerPawn` 0)))))
  (`|ExecutionSequence`
    (:`then_0`
      ; Spawn disappearing text
      (`|SpawnActorFromClass` "/Game/FrontierDestiny/99_Testing/BP_DisappearingText.BP_DisappearingText_C" (`KismetMathLibrary.MakeTransform` (+ (* (`KismetMathLibrary.GetRightVector` _returnvalue) (`KismetMathLibrary.RandomFloatInRange` 0.0 50.0)) (* (`KismetMathLibrary.GetUpVector` _returnvalue) (`KismetMathLibrary.RandomFloatInRange` 0.0 50.0)) (+ _location (0.0 0.0 100.0))) _returnvalue (.scale (`self.GetTransform`))) "AlwaysSpawn" "MultiplyWithRoot" (`self.GetOwner`) (`KismetTextLibrary.Conv_DoubleToText` Damage "HalfToEven") (`self.GetInstigator`)))))

(fn `UserConstructionScript`)