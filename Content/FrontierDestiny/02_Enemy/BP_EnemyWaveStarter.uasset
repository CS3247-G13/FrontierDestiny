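; Blueprint that starts enemy hordes through the EnemyWaveManager subsystem in response to quest progress.
; On BeginPlay it binds to quest updates and horde-finished events.
; When the current quest becomes Horde_1 it starts the first horde, and that horde's completion starts the second after a three-minute delay.
; Each trigger fires once, and every quest update prints the current quest ID.
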(event `On Horde Finish`
  (params (HordeID :type Name))
  (if (== HordeID "0")
    (`/Engine/EditorBlueprintResources/StandardMacros.DoOnce` false
      (:`Completed`
        (`KismetSystemLibrary.Delay` 180.0)
        (`EnemyWaveManagerSubsystem.StartHorde` (subsystem `EnemyWaveManagerSubsystem`) "1")))))

(event `self.ReceiveBeginPlay`
  (add `QuestSubsystem.OnQuestUpdated` (subsystem `QuestSubsystem`) (delegate `On Quest`))
  (add `EnemyWaveManagerSubsystem.OnHordeFinished` (subsystem `EnemyWaveManagerSubsystem`) (delegate `On Horde Finish`)))

(event `On Quest`
  (bind _currentquest_questid (break `QuestData` (`QuestSubsystem.CurrentQuest` (subsystem `QuestSubsystem`))))
  (`KismetSystemLibrary.PrintString` (`KismetStringLibrary.Conv_NameToString` _currentquest_questid))
  (if (== _currentquest_questid "Horde_1")
    (`/Engine/EditorBlueprintResources/StandardMacros.DoOnce` false
      (:`Completed`
        (`EnemyWaveManagerSubsystem.StartHorde` (subsystem `EnemyWaveManagerSubsystem`) "0")))))

(fn `UserConstructionScript`)