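; Beam Threader tower that periodically fires a piercing laser, damaging and burning enemies along its line.
; It rotates to face a target from the enemy manager subsystem, reselecting when that target is invalid, dies or leaves range or sight.
; A looping cooldown triggers a forward sphere trace to full range, spawning a Niagara beam and sound.
; Traced unique enemies take stat-driven laser damage and burn after a short delay, then the tower retargets.
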(event `self.OnTowerActive`
  (bind _cooldown (`self.Cooldown`))
  (`|ExecutionSequence`
    (:`then_0`
      ; Start cooldown
      (set `CooldownComponent.CooldownDuration` (`.Cooldown` (break `TowerData` (`self.TowerData`))) _cooldown)
      (`CooldownComponent.StartCooldown` _cooldown)
      (set `CooldownComponent.Mode` "LoopOnFinish" _cooldown))
    (:`then_1`
      (add `CooldownComponent.OnCooldownFinished` (`self.Cooldown`) (delegate `OnCooldownFinished_Event`)))
    (:`then_2`
      (if (not (`EnemyManagerSubsystem.IsTargetValid` (subsystem `EnemyManagerSubsystem`) (`self.CurrentTarget`)))
        (`self.SelectTarget`)))))

(event `self.OnTowerTick`
  (params (DeltaTime :type "Float (single-precision)"))
  (bind _returnvalue (subsystem `EnemyManagerSubsystem`))
  (bind _currenttarget (`self.CurrentTarget`))
  (if (`EnemyManagerSubsystem.IsTargetValid` _returnvalue _currenttarget)
    ; Rotate
    (`TowerBlueprintFunctionLibrary.RotateTowerToFace` (`self.Joint`) (`self.Body`) (`EnemyManagerSubsystem.GetTargetPosition` _returnvalue _currenttarget) (`self.GetStats` (struct :`TagName` "Tower.Movement.RotationSpeed")) DeltaTime)
    (else
      (`self.SelectTarget`))))

(event `OnCooldownFinished_Event`
  (if (`EnemyManagerSubsystem.IsTargetValid` (subsystem `EnemyManagerSubsystem`) (`self.CurrentTarget`))
    (bind (_beam _targets) (`self.FireLaser`))
    (`KismetSystemLibrary.Delay` 0.4)
    (`self.DamageEnemies` _targets)
    (`self.SelectTarget`)))

(event `self.OnTargetEnterRange`
  (params (Target :type "MassEnemyTarget Structure"))
  (if (not (`EnemyManagerSubsystem.IsTargetValid` (subsystem `EnemyManagerSubsystem`) (`self.CurrentTarget`)))
    (`self.SelectTarget` :!label _label)))

(event `self.OnTargetLeaveRange`
  (params (Target :type "MassEnemyTarget Structure"))
  (goto _label))

(event `self.OnAcquireNewTarget`
  (params (Target :type "MassEnemyTarget Structure")))

(event `self.OnTargetDeath`
  (goto _label))

(event `self.LoseSightOfTarget`
  (goto _label))

(fn `CheckTargetVisible`
  (params (Target :type "MassEnemyTarget Structure"))
  (returns (ReturnValue :type Boolean))
  (bind _returnvalue (`TowerBlueprintFunctionLibrary.CheckEnemyVisibleFromPoint` (`SceneComponent.K2_GetComponentLocation` (`self.Scene`)) Target (`|MakeArray` self :!type "Actor Object Reference")))
  (return _returnvalue))

(fn `DamageEnemies`
  (params (Target :type "Array of MassEnemyTarget Structure"))
  (bind _returnvalue (subsystem `EnemyManagerSubsystem`))
  (for _array_element Target
    (`EnemyManagerSubsystem.ApplyDamageToTarget` _returnvalue _array_element (`KismetMathLibrary.FTrunc` (`self.GetStats` (struct :`TagName` "Tower.Damage.BaseDamage"))) (`.Position` (break `MassEnemyTarget` _array_element)) "Laser")
    (`EnemyManagerSubsystem.ApplyBurn` _returnvalue _array_element (`self.GetStats` (struct :`TagName` "Tower.Damage.DOT.Duration")) (`self.GetStats` (struct :`TagName` "Tower.Damage.DOT.DamagePerTick")) (`self.GetStats` (struct :`TagName` "Tower.Damage.DOT.TickInterval")))))

(fn `FireLaser`
  (returns (Beam :type "NiagaraComponent Object Reference") (Targets :type "Array of MassEnemyTarget Structure"))
  (bind _returnvalue (`SceneComponent.K2_GetComponentLocation` (`self.Scene`)))
  (bind _returnvalue_2 (`KismetMathLibrary.Conv_IntToDouble` (`.Range` (break `TowerData` (`self.TowerData`)))))
  (bind _returnvalue_3 (+ (* (`SceneComponent.GetForwardVector` (`self.Body`)) _returnvalue_2) _returnvalue))
  (bind _outhits (`KismetSystemLibrary.SphereTraceMulti` :`Start` _returnvalue :`End` _returnvalue_3 :`Radius` 10.0 :`TraceChannel` "TraceTypeQuery5" :`DrawTime` 1.0))
  (bind _returnvalue_4 (`TowerBlueprintFunctionLibrary.GetUniqueEnemyTargetsFromHits` _outhits (`|MakeArray` (struct) :!type "MassEnemyTarget Structure")))
  (bind _beam (`self.SpawnBeam` _returnvalue _returnvalue_3 _returnvalue_2))
  (`GameplayStatics.PlaySoundAtLocation` "/Game/FrontierDestiny/03_Tower/Audio/BeamThreader_Fire.BeamThreader_Fire" _returnvalue (struct) 1.0 1.0 0.0 "/Game/FrontierDestiny/03_Tower/Audio/TowerAttenuation.TowerAttenuation" null null null)
  (return _beam _returnvalue_4))

(fn `SpawnBeam`
  (params (Origin :type "Vector Structure") (Target :type "Vector Structure") (Range :type "Float (double-precision)"))
  (returns (Beam :type "NiagaraComponent Object Reference"))
  (bind _returnvalue (`NiagaraFunctionLibrary.SpawnSystemAtLocation` "/Game/FrontierDestiny/Levels/ParticleEffects/NS_ThreaderBeam.NS_ThreaderBeam"))
  (`NiagaraComponent.SetVariableVec3` _returnvalue "Origin" Origin)
  (`NiagaraComponent.SetVariableVec3` _returnvalue "Target" Target)
  (`NiagaraComponent.SetNiagaraVariableFloat` _returnvalue "Range" Range)
  (return _returnvalue))

(fn `UserConstructionScript`)