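; Lightning variant of a beam Threader tower that adds chaining electric area damage to its attack.
; After the parent damage step, it sphere-traces around each hit enemy for new targets, spawning Niagara arcs and dealing Electric damage through the enemy manager subsystem.
; New targets are appended to the list being iterated, so arcs keep chaining without repeat hits.
; SpawnBeam supplies the lightning beam effect with origin, target and range.
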(fn `DamageEnemies`
  (params (Target :type "Array of MassEnemyTarget Structure (by ref)"))
  (locals (`All Hits` :type "Array of MassEnemyTarget Structure"))
  (`parent.DamageEnemies` Target)
  (bind _output_get (set `local.All Hits` Target))
  (for _array_element _output_get
    (bind _position (break `MassEnemyTarget` _array_element))
    (bind _outhits (`KismetSystemLibrary.SphereTraceMulti` :`Start` _position :`End` _position :`Radius` (`self.GetStats` (struct :`TagName` "Tower.Damage.AOE.Radius")) :`TraceChannel` "TraceTypeQuery5" :`DrawTime` 2.0))
    (bind _returnvalue (`TowerBlueprintFunctionLibrary.GetUniqueEnemyTargetsFromHits` _outhits _output_get))
    (for _array_element_2 _returnvalue
      (bind _position_2 (break `MassEnemyTarget` _array_element_2))
      (bind _returnvalue_2 (`NiagaraFunctionLibrary.SpawnSystemAtLocation` "/Game/FrontierDestiny/Levels/ParticleEffects/NS_Lightning_Arc.NS_Lightning_Arc" _position_2))
      (`NiagaraComponent.SetVariablePosition` _returnvalue_2 "Origin" _position)
      (`NiagaraComponent.SetVariablePosition` _returnvalue_2 "Target" _position_2)
      (`EnemyManagerSubsystem.ApplyDamageToTarget` (subsystem `EnemyManagerSubsystem`) _array_element_2 (`KismetMathLibrary.FTrunc` (`self.GetStats` (struct :`TagName` "Tower.Damage.AOE.BaseDamage"))) _position_2 "Electric"))
    (`KismetArrayLibrary.Array_Append` _output_get _returnvalue))
  (return))

(fn `SpawnBeam`
  (params (Origin :type "Vector Structure") (Target :type "Vector Structure") (Range :type "Float (double-precision)"))
  (returns (Beam :type "NiagaraComponent Object Reference"))
  (bind _returnvalue (`NiagaraFunctionLibrary.SpawnSystemAtLocation` "/Game/FrontierDestiny/Levels/ParticleEffects/NS_ThreaderLightning.NS_ThreaderLightning"))
  (`NiagaraComponent.SetVariableVec3` _returnvalue "Origin" Origin)
  (`NiagaraComponent.SetVariableVec3` _returnvalue "Target" Target)
  (`NiagaraComponent.SetNiagaraVariableFloat` _returnvalue "Range" Range)
  (return _returnvalue))

(fn `UserConstructionScript`
  (`parent.UserConstructionScript`))