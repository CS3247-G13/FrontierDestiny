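; BP_IonisedSnare is an ionised Tremor Snare tower variant that damages and stuns enemies.
; DamageEnemy sends truncated base-damage Kinetic hits and a stun to the EnemyManagerSubsystem, reading damage and stun duration from tagged tower stats.
; SpawnEmitter plays the NS_IonizedTremor Niagara effect at a given origin.
; The event graph is empty, so nothing in this Blueprint calls either function itself.
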(fn `DamageEnemy`
  (params (Target :type "MassEnemyTarget Structure") (`Imapct Location` :type "Vector Structure"))
  (bind _returnvalue (subsystem `EnemyManagerSubsystem`))
  (`|ExecutionSequence`
    (:`then_1`
      (`EnemyManagerSubsystem.ApplyDamageToTarget` _returnvalue Target (`KismetMathLibrary.FTrunc` (`self.GetStats` (struct :`TagName` "Tower.Damage.BaseDamage"))) `Imapct Location` "Kinetic")
      (`EnemyManagerSubsystem.ApplyStun` _returnvalue Target (`self.GetStats` (struct :`TagName` "Tower.Utility.StunDuration"))))))

(fn `SpawnEmitter`
  (params (Origin :type "Vector Structure"))
  (`NiagaraFunctionLibrary.SpawnSystemAtLocation` "/Game/FrontierDestiny/Levels/ParticleEffects/NS_IonizedTremor.NS_IonizedTremor" Origin))

(fn `UserConstructionScript`
  (`parent.UserConstructionScript`))