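; Phase Wall tower Blueprint that retaliates against attackers by damaging the pawn behind any damage it takes.
; On AnyDamage, it applies the base damage from its TowerData effects to the instigator's controlled pawn, credited to the tower's instigator controller.
; DamageableMap gates retaliation per pawn, blocking repeat hits until a single shared Delay of the tower's cooldown re-enables the pawn.
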(event `self.ReceiveAnyDamage`
  (params (Damage :type "Float (single-precision)") (DamageType :type "DamageType Object Reference") (InstigatedBy :type "Controller Object Reference") (DamageCauser :type "Actor Object Reference"))
  (bind _returnvalue (`Controller.K2_GetPawn` InstigatedBy))
  (bind _returnvalue_2 (`self.GetInstigatorController`))
  (bind (_value _returnvalue_3) (`BlueprintMapLibrary.Map_Find` (`self.DamageableMap`) _returnvalue))
  (`/Engine/EditorBlueprintResources/StandardMacros.IsValid` InstigatedBy
    (:`Is Valid`
      (`/Engine/EditorBlueprintResources/StandardMacros.IsValid` _returnvalue
        (:`Is Valid`
          (if (or _value (not _returnvalue_3))
            (`/Engine/EditorBlueprintResources/StandardMacros.IsValid` _returnvalue_2
              (:`Is Valid`
                (`GameplayStatics.ApplyDamage` _returnvalue (`.Amount` (break `TowerEffect` (`BlueprintMapLibrary.Map_Find` (`.Effects` (break `TowerData` (`self.TowerData`))) (struct :`TagName` "Tower.Damage.BaseDamage")))) _returnvalue_2 self)
                (`BlueprintMapLibrary.Map_Add` (`self.DamageableMap`) _returnvalue)
                (`KismetSystemLibrary.Delay` (`.Cooldown` (break `TowerData` (`self.TowerData`))))
                (`BlueprintMapLibrary.Map_Add` (`self.DamageableMap`) _returnvalue true)))))))))

(fn `UserConstructionScript`)