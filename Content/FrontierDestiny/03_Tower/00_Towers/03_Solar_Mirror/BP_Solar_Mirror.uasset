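; Solar Mirror tower that fires a continuous Niagara laser at one enemy, with damage ramping up the longer it stays on target.
; A looping timer applies damage and raises it toward a stat-driven cap, while tower tick widens the beam in step with the ramp.
; Losing the target through death, range or line of sight resets damage and plays a timeline that shrinks the beam from its current width before retargeting.
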(event `self.OnTowerActive`
  (bind _scene (`self.Scene`))
  (bind _returnvalue (`SceneComponent.K2_GetComponentLocation` _scene))
  (`|ExecutionSequence`
    (:`then_0`
      (bind _returnvalue_2 (`self.GetStats` (struct :`TagName` "Tower.SolarMirror.Laser.MaxDamage")))
      (bind _returnvalue_3 (`self.GetStats` (struct :`TagName` "Tower.Damage")))
      (bind _returnvalue_4 (`self.GetStats` (struct :`TagName` "Tower.SolarMirror.Laser.TickDamageIncrease")))
      (bind _returnvalue_5 (`self.GetStats` (struct :`TagName` "Tower.SolarMirror.Laser.TickLength")))
      (set `self.Max Ramp Duration` (* (/ (- _returnvalue_2 _returnvalue_3) _returnvalue_4) _returnvalue_5)))
    (:`then_1`
      (bind _returnvalue_6 (`NiagaraFunctionLibrary.SpawnSystemAtLocation` "/Game/FrontierDestiny/Levels/ParticleEffects/NS_SolarRay.NS_SolarRay" _returnvalue (`SceneComponent.K2_GetComponentRotation` _scene) (`SceneComponent.K2_GetComponentScale` _scene) false false))
      (bind _output_get (set `self.Laser Particle` _returnvalue_6))
      (`ActorComponent.Activate` _output_get true)
      (`NiagaraComponent.SetVariableVec3` _output_get "Origin" _returnvalue)
      (`NiagaraComponent.SetVariableVec3` _output_get "Target" (0.0 0.0 0.0))
      ; Choose a target
      (`self.SelectTarget`)
      (bind _returnvalue_7 (`self.GetStats` (struct :`TagName` "Tower.Damage")))
      (set `self.Current Damage` _returnvalue_7))))

(event `self.OnTowerTick`
  (params (DeltaTime :type "Float (single-precision)"))
  (`|ExecutionSequence`
    (:`then_0`
      (if (`self.ShouldUpdateLaser`)
        (`self.Update Laser Size And Location`)))
    (:`then_1`
      ; Select target if laser has powered down
      (if (`self.SearchingForNewTarget`) :!label _label
        (`self.SelectTarget`)))
    (:`then_2`
      (set `self.Ramp Duration` (`KismetMathLibrary.FMin` (+ DeltaTime (`self.Ramp Duration`)) (`self.Max Ramp Duration`))))))

(event `self.OnTargetEnterRange`
  (params (Target :type "MassEnemyTarget Structure"))
  (goto _label))

(event `Power Down Laser`
  (bind _returnvalue (`self.GetStats` (struct :`TagName` "Tower.Damage")))
  (set `self.Current Damage` _returnvalue)
  (set `self.ShouldUpdateLaser` false)
  (bind _width (`self.Get Laser Width`))
  (`|ExecutionSequence`
    (:`then_0`
      (bind (_direction _power_down_track) (`Timeline|PowerdownTimeline` :`NewTime` (- 1.0 _width) :!via `SetNewTime` :!label _label_2)
        (:`Update`
          (`NiagaraComponent.SetVariableFloat` (`self.Laser Particle`) "Beam Width Scale" _power_down_track))
        (:`Finished`
          (set `self.SearchingForNewTarget` true)
          (`self.SelectTarget`))))
    (:`then_1`
      (goto _label_2))))

(event `self.OnTargetLeaveRange`
  (params (Target :type "MassEnemyTarget Structure"))
  ; Select target if target left range
  (if (`EnemyManagerSubsystem.IsSameTarget` (subsystem `EnemyManagerSubsystem`) Target (`self.CurrentTarget`))
    (`self.Reset Laser` :!label _label_3)))

(event `self.OnAcquireNewTarget`
  (params (Target :type "MassEnemyTarget Structure"))
  (set `self.ShouldUpdateLaser` true)
  (bind _returnvalue (`self.GetStats` (struct :`TagName` "Tower.SolarMirror.Laser.TickLength")))
  (set `self.Ramp Duration` 0.0)
  (set `self.SearchingForNewTarget` false)
  (bind _returnvalue_2 (`KismetSystemLibrary.K2_SetTimer` null "Damage And Update Laser Damage" _returnvalue true))
  (set `self.Damage Update Timer` _returnvalue_2))

(event `self.OnTargetDeath`
  (goto _label_3))

(event `self.LoseSightOfTarget`
  (goto _label_3))

(fn `CheckTargetVisible`
  (params (Target :type "MassEnemyTarget Structure"))
  (returns (ReturnValue :type Boolean))
  (bind _returnvalue (subsystem `EnemyManagerSubsystem`))
  (bind _outhit (`KismetSystemLibrary.LineTraceSingle` (`SceneComponent.K2_GetComponentLocation` (`self.Scene`)) (`.Position` (break `MassEnemyTarget` Target)) "TraceTypeQuery1" false (`|MakeArray` self :!type "Actor Object Reference")))
  (bind (_outtarget _returnvalue_2) (`EnemyManagerSubsystem.GetEnemyTargetFromHit` _returnvalue _outhit))
  (return (and _returnvalue_2 (`EnemyManagerSubsystem.IsSameTarget` _returnvalue _outtarget Target))))

(fn `Damage And Update Laser Damage`
  (`|ExecutionSequence`
    (:`then_0`
      (if (`EnemyManagerSubsystem.IsTargetValid` (subsystem `EnemyManagerSubsystem`) (`self.CurrentTarget`))
        (`EnemyManagerSubsystem.ApplyDamageToTarget` (subsystem `EnemyManagerSubsystem`) (`self.CurrentTarget`) (`KismetMathLibrary.FTrunc` (`self.Current Damage`)))))
    (:`then_1`
      (bind _returnvalue (`self.GetStats` (struct :`TagName` "Tower.SolarMirror.Laser.TickDamageIncrease")))
      (bind _returnvalue_2 (`self.GetStats` (struct :`TagName` "Tower.SolarMirror.Laser.MaxDamage")))
      (set `self.Current Damage` (`KismetMathLibrary.FMin` (+ _returnvalue (`self.Current Damage`)) _returnvalue_2)))))

(fn `Get Laser Width`
  (returns (Width :type "Float (double-precision)"))
  (return (`KismetMathLibrary.FClamp` (/ (`self.Ramp Duration`) (`self.Max Ramp Duration`)))))

(fn `Reset Laser`
  (`KismetSystemLibrary.K2_ClearAndInvalidateTimerHandle` (`self.Damage Update Timer`))
  (`self.Power Down Laser`))

(fn `Update Laser Size And Location`
  (bind _currenttarget (`self.CurrentTarget`))
  (if (`EnemyManagerSubsystem.IsTargetValid` (subsystem `EnemyManagerSubsystem`) _currenttarget)
    (`NiagaraComponent.SetVariableVec3` (`self.Laser Particle`) "Target" (`.Position` (break `MassEnemyTarget` _currenttarget)))
    (bind _width (`self.Get Laser Width`))
    (`NiagaraComponent.SetVariableFloat` (`self.Laser Particle`) "Beam Width Scale" _width)))

(fn `UserConstructionScript`)