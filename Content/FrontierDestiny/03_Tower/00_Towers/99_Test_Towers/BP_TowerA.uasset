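; BP_TowerA is a test tower that turns its head toward the current target and fires bullets on a cooldown.
; On activation it starts the cooldown from TowerData; each finish attempts an attack and restarts the cooldown only on success.
; An attack spawns BP_Bullet at Spawnpoint along the head's forward vector, with base damage looked up by gameplay tag.
; Each tick, the head slerps toward the target's "Target"-tagged component.
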(event `self.OnTowerActive`
  (bind _cooldown (`self.Cooldown`))
  ; Begin Cooldown
  (set `CooldownComponent.CooldownDuration` (`.Cooldown` (break `TowerData` (`self.TowerData`))) _cooldown)
  (`CooldownComponent.StartCooldown` _cooldown))

(event `self.Cooldown.OnCooldownFinished`
  (bind _cooldown (`self.Cooldown`))
  ; Try to attack, if it succeeds, reset the cooldown
  (bind _success (`self.TryAttackEnemy`))
  (if _success
    (`CooldownComponent.ResetCooldown` _cooldown)
    (`CooldownComponent.StartCooldown` _cooldown)))

(event `self.OnTowerTick`
  (params (DeltaTime :type "Float (single-precision)"))
  (bind _towera_head (`self.TowerA_Head`))
  ; Rotate the tower to face the enemy
  (if (not (`self.TargetIsNull`))
    (`SceneComponent.K2_SetWorldRotation` (`self.TowerA_Head`) (`TowerUtilities.QuaternionSlerp` (`SceneComponent.K2_GetComponentRotation` _towera_head) (`KismetMathLibrary.MakeRotFromX` (`KismetMathLibrary.GetDirectionUnitVector` (`SceneComponent.K2_GetComponentLocation` _towera_head) (`SceneComponent.K2_GetComponentLocation` (`|GetArrayItem` (`self.GetComponentsByTag` (`self.CurrentTarget`) "/Script/Engine.SceneComponent" "Target"))))) DeltaTime (`self.HeadRotationalSpeed`)) false false)))

(fn `TryAttackEnemy`
  (returns (Success :type Boolean))
  (if (not (`self.TargetIsNull`))
    (`|SpawnActorFromClass` "/Game/FrontierDestiny/03_Tower/00_Towers/99_Test_Towers/Projectiles/BP_Bullet.BP_Bullet_C" (`SceneComponent.K2_GetComponentToWorld` (`self.Spawnpoint`)) "AlwaysSpawn" "OverrideRootScale" self (`.Amount` (break `TowerEffect` (`BlueprintMapLibrary.Map_Find` (`.Effects` (break `TowerData` (`self.TowerData`))) (struct :`TagName` "Tower.Damage.BaseDamage")))) (`SceneComponent.GetForwardVector` (`self.TowerA_Head`)) 30000.0 (`self.GetInstigator`))
    (return true)))

(fn `UserConstructionScript`)