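; Crusher tower Blueprint that periodically slams down to deal kinetic damage and apply a slow to nearby enemies.
; A cooldown, started on tower activation, triggers Thump, whose timelines lerp the crusher mesh between Low and High points.
; On landing it plays a sound and sphere-traces the tower's range, de-duplicating targets through the EnemyManager subsystem.
; Only targets within the height limit are hit, then a second timeline raises the crusher.
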(event `self.ReceiveBeginPlay`)

(event `Thump`
  (bind _returnvalue (subsystem `EnemyManagerSubsystem`))
  (bind _returnvalue_2 (`SceneComponent.K2_GetComponentLocation` (`self.RangeComponent`)))
  (bind _returnvalue_3 (`SceneComponent.K2_GetComponentLocation` (`self.Low`)))
  ; Go down
  (bind (_direction _down) (`Timeline|Down Movement` :!via `PlayFromStart`)
    (:`Update`
      (`SceneComponent.K2_SetWorldLocation` (`self.SM_Crusher_A`) (`KismetMathLibrary.VLerp` _returnvalue_3 (`SceneComponent.K2_GetComponentLocation` (`self.High`)) _down) false false))
    (:`Finished`
      (`GameplayStatics.PlaySoundAtLocation` "/Game/FrontierDestiny/03_Tower/Audio/TremorSnare_Slam_3.TremorSnare_Slam_3" _returnvalue_3 (struct) 2.0 1.0 0.0 null null null null)
      (bind _outhits (`KismetSystemLibrary.SphereTraceMulti` _returnvalue_2 _returnvalue_2 (`KismetMathLibrary.Conv_IntToDouble` (`.Range` (break `TowerData` (`self.TowerData`)))) "TraceTypeQuery5"))
      (`KismetArrayLibrary.Array_Clear` (`self.EnemiesHit`))
      (for _array_element _outhits
        (bind (_outtarget _returnvalue_4) (`EnemyManagerSubsystem.GetEnemyTargetFromHit` _returnvalue _array_element))
        (if _returnvalue_4
          (bind _output_get (set `self.Exists` false))
          (for _array_element_2 (`self.EnemiesHit`)
            (if (`EnemyManagerSubsystem.IsSameTarget` _returnvalue _outtarget _array_element_2)
              (set `self.Exists` true)
              (break)))
          (if (not _output_get)
            (`KismetArrayLibrary.Array_Add` (`self.EnemiesHit`) _outtarget)
            ; Check target is below height
            (if (<= (.z (- (`.Position` (break `MassEnemyTarget` _outtarget)) (`SceneComponent.K2_GetComponentLocation` (`self.RangeComponent`)))) (`self.GetStats` (struct :`TagName` "Tower.TremorSnare.Height")))
              (`self.DamageEnemy` _outtarget (`.ImpactPoint` (`GameplayStatics.BreakHitResult` _array_element)))))))
      ; Go up
      (bind (_direction_2 _up) (`Timeline|Timeline` :!via `PlayFromStart`)
        (:`Update`
          (`SceneComponent.K2_SetWorldLocation` (`self.SM_Crusher_A`) (`KismetMathLibrary.VLerp` (`SceneComponent.K2_GetComponentLocation` (`self.Low`)) (`SceneComponent.K2_GetComponentLocation` (`self.High`)) _up) false false))))))

(event `self.OnTargetEnterRange`
  (params (Target :type "MassEnemyTarget Structure")))

(event `self.OnTargetLeaveRange`
  (params (Target :type "MassEnemyTarget Structure")))

(event `self.OnTowerActive`
  (bind _cooldown (`self.Cooldown`))
  (set `CooldownComponent.CooldownDuration` (`.Cooldown` (break `TowerData` (`self.TowerData`))) _cooldown)
  (`CooldownComponent.StartCooldown` _cooldown)
  (add `CooldownComponent.OnCooldownFinished` _cooldown (delegate `OnCooldownFinished_Event`))
  (`self.OnCooldownFinished_Event`))

(event `OnCooldownFinished_Event`
  (bind _cooldown (`self.Cooldown`))
  (`CooldownComponent.ResetCooldown` _cooldown)
  (`CooldownComponent.StartCooldown` _cooldown)
  (`self.Thump`))

(event `self.OnTowerTick`
  (params (DeltaTime :type "Float (single-precision)")))

(fn `DamageEnemy`
  (params (Target :type "MassEnemyTarget Structure") (`Imapct Location` :type "Vector Structure"))
  (bind _returnvalue (subsystem `EnemyManagerSubsystem`))
  (`|ExecutionSequence`
    (:`then_1`
      (`EnemyManagerSubsystem.ApplyDamageToTarget` _returnvalue Target (`KismetMathLibrary.FTrunc` (`self.GetStats` (struct :`TagName` "Tower.Damage.BaseDamage"))) `Imapct Location` "Kinetic")
      (`EnemyManagerSubsystem.ApplySlow` _returnvalue Target (`self.GetStats` (struct :`TagName` "Tower.Utility.SlowDuration")) (`self.GetStats` (struct :`TagName` "Tower.Utility.SlowAmount"))))))

(fn `UserConstructionScript`)