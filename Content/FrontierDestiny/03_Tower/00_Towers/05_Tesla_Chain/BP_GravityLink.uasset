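; BP_GravityLink is a chain tower variant in the Tesla Chain family that slows the enemies it damages.
; It extends the parent's main and peripheral enemy damage functions, running the parent damage first and then calling SlowEnemy on the same target.
; SlowEnemy applies the slow through the EnemyManagerSubsystem, with duration and amount read from the tower's Utility stat tags.
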(fn `DamageMainEnemy`
  (params (Target :type "MassEnemyTarget Structure"))
  (`parent.DamageMainEnemy` Target)
  (`self.SlowEnemy` Target))

(fn `DamagePeripheralEnemy`
  (params (Target :type "MassEnemyTarget Structure"))
  (`parent.DamagePeripheralEnemy` Target)
  (`self.SlowEnemy` Target))

(fn `SlowEnemy`
  (params (Target :type "MassEnemyTarget Structure"))
  (`EnemyManagerSubsystem.ApplySlow` (subsystem `EnemyManagerSubsystem`) Target (`self.GetStats` (struct :`TagName` "Tower.Utility.SlowDuration")) (`self.GetStats` (struct :`TagName` "Tower.Utility.SlowAmount"))))

(fn `UserConstructionScript`
  (`parent.UserConstructionScript`))