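; Tesla chain tower that periodically shocks enemies with electric damage, with lightning chaining from each target to a nearby one.
; On each cooldown it selects targets by its Targets stat, damages them and draws Niagara arcs from the Bulb.
; A sphere trace around each target finds one enemy not yet hit this volley, which takes separate AOE damage via EnemyManagerSubsystem and gets an arc from the main target.
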(event `self.OnTowerActive`
  (bind _cooldown (`self.Cooldown`))
  (set `CooldownComponent.CooldownDuration` (`.Cooldown` (break `TowerData` (`self.TowerData`))) _cooldown)
  (`CooldownComponent.StartCooldown` _cooldown)
  (add `CooldownComponent.OnCooldownFinished` _cooldown (delegate `OnCooldownFinished_Event`))
  (`self.OnCooldownFinished_Event`))

(event `OnCooldownFinished_Event`
  (bind _cooldown (`self.Cooldown`))
  (`CooldownComponent.ResetCooldown` _cooldown)
  (`CooldownComponent.StartCooldown` _cooldown)
  (bind _output_get (set `self.SelectedTargets` (`self.SelectTargets` (`KismetMathLibrary.FTrunc` (`self.GetStats` (struct :`TagName` "Tower.Targets"))))))
  (set `self.TargetsAttacked` _output_get)
  (for _array_element (`self.SelectedTargets`)
    (bind _position (break `MassEnemyTarget` _array_element))
    (bind _arc (`self.SpawnArc` _position))
    (`NiagaraComponent.SetVariablePosition` _arc "Origin" (`SceneComponent.K2_GetComponentLocation` (`self.Bulb`)))
    (`NiagaraComponent.SetVariablePosition` _arc "Target" _position)
    (`self.DamageMainEnemy` _array_element)
    (bind _position_2 (break `MassEnemyTarget` _array_element))
    (bind _outhits (`KismetSystemLibrary.SphereTraceMulti` :`Start` _position_2 :`End` _position_2 :`Radius` (`self.GetStats` (struct :`TagName` "Tower.Damage.AOE.Radius")) :`TraceChannel` "TraceTypeQuery5" :`TraceColor` (struct :`R` 0.994667 :`G` 0.001738 :`B` 1.0 :`A` 1.0) :`TraceHitColor` (struct :`G` 0.155987 :`B` 1.0 :`A` 1.0)))
    (bind _returnvalue (`TowerBlueprintFunctionLibrary.GetUniqueEnemyTargetsFromHits` _outhits (`self.TargetsAttacked`)))
    (for _array_element_2 _returnvalue
      (bind _position_3 (break `MassEnemyTarget` _array_element_2))
      (bind _arc_2 (`self.SpawnArc` _position_3))
      (`NiagaraComponent.SetVariablePosition` _arc_2 "Origin" _position_2)
      (`NiagaraComponent.SetVariablePosition` _arc_2 "Target" _position_3)
      (`self.DamagePeripheralEnemy` _array_element_2)
      (`KismetArrayLibrary.Array_Append` (`self.TargetsAttacked`) (`|MakeArray` _array_element_2))
      (break))))

(fn `DamageMainEnemy`
  (params (Target :type "MassEnemyTarget Structure"))
  (`EnemyManagerSubsystem.ApplyDamageToTarget` (subsystem `EnemyManagerSubsystem`) Target (`KismetMathLibrary.FTrunc` (`self.GetStats` (struct :`TagName` "Tower.Damage.BaseDamage"))) (`.Position` (break `MassEnemyTarget` Target)) "Electric"))

(fn `DamagePeripheralEnemy`
  (params (Target :type "MassEnemyTarget Structure"))
  (`EnemyManagerSubsystem.ApplyDamageToTarget` (subsystem `EnemyManagerSubsystem`) Target (`KismetMathLibrary.FTrunc` (`self.GetStats` (struct :`TagName` "Tower.Damage.AOE.BaseDamage"))) (`.Position` (break `MassEnemyTarget` Target)) "Electric"))

(fn `SpawnArc`
  (params (Origin :type "Vector Structure"))
  (returns (Arc :type "NiagaraComponent Object Reference"))
  (bind _returnvalue (`NiagaraFunctionLibrary.SpawnSystemAtLocation` "/Game/FrontierDestiny/Levels/ParticleEffects/NS_Lightning_Arc.NS_Lightning_Arc" Origin))
  (return _returnvalue))

(fn `UserConstructionScript`)