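; Beam Threader tower that fires a piercing laser, damaging every enemy along a straight line out to the tower's range.
; Each tick it slerps the joint's yaw and body's pitch toward the current target, reselecting when that target is invalid.
; A looping cooldown triggers a debug-drawn sphere trace along the body's forward vector, applying base damage to deduplicated hits via EnemyManagerSubsystem.
; CheckTargetVisible tests line of sight; damage-over-time code is disconnected.
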(event `self.OnTowerActive`
  (bind _cooldown (`self.Cooldown`))
  (`|ExecutionSequence`
    (:`then_0`
      ; Start cooldown
      (set `CooldownComponent.CooldownDuration` (`.Cooldown` (break `TowerData` (`self.TowerData`))) _cooldown)
      (`CooldownComponent.StartCooldown` _cooldown)
      (set `CooldownComponent.Mode` "LoopOnFinish" _cooldown))
    (:`then_1`
      (add `CooldownComponent.OnCooldownFinished` (`self.Cooldown`) (delegate `OnCooldownFinished_Event`)))
    (:`then_2`
      (if (not (`EnemyManagerSubsystem.IsTargetValid` (subsystem `EnemyManagerSubsystem`) (`self.CurrentTarget`)))
        (`self.SelectTarget`)))))

(event `self.OnTowerTick`
  (params (DeltaTime :type "Float (single-precision)"))
  (if (`EnemyManagerSubsystem.IsTargetValid` (subsystem `EnemyManagerSubsystem`) (`self.CurrentTarget`))
    ; Rotate
    (`SceneComponent.K2_SetWorldRotation` (`self.Joint`) (`KismetMathLibrary.MakeRotator` 0.0 0.0 (.yaw (`TowerUtilities.QuaternionSlerp` (`KismetMathLibrary.MakeRotator` 0.0 (.pitch (`SceneComponent.RelativeRotation` (`self.Body`))) (.yaw (`SceneComponent.K2_GetComponentRotation` (`self.Joint`)))) (`KismetMathLibrary.MakeRotFromX` (`KismetMathLibrary.GetDirectionUnitVector` (`SceneComponent.K2_GetComponentLocation` (`self.Body`)) (`.Position` (break `MassEnemyTarget` (`self.CurrentTarget`))))) DeltaTime (`self.RotationSpeed`)))) false false)
    (`SceneComponent.K2_SetRelativeRotation` (`self.Body`) (`KismetMathLibrary.MakeRotator` 0.0 (.pitch (`TowerUtilities.QuaternionSlerp` (`KismetMathLibrary.MakeRotator` 0.0 (.pitch (`SceneComponent.RelativeRotation` (`self.Body`))) (.yaw (`SceneComponent.K2_GetComponentRotation` (`self.Joint`)))) (`KismetMathLibrary.MakeRotFromX` (`KismetMathLibrary.GetDirectionUnitVector` (`SceneComponent.K2_GetComponentLocation` (`self.Body`)) (`.Position` (break `MassEnemyTarget` (`self.CurrentTarget`))))) DeltaTime (`self.RotationSpeed`)))) false false)
    (else
      (`self.SelectTarget`))))

(event `OnCooldownFinished_Event`
  (if (`EnemyManagerSubsystem.IsTargetValid` (subsystem `EnemyManagerSubsystem`) (`self.CurrentTarget`))
    (`self.FireLaser`)
    (`self.SelectTarget`)))

(event `self.OnTargetEnterRange`
  (params (Target :type "MassEnemyTarget Structure"))
  (if (not (`EnemyManagerSubsystem.IsTargetValid` (subsystem `EnemyManagerSubsystem`) (`self.CurrentTarget`)))
    (`self.SelectTarget` :!label _label)))

(event `self.OnTargetLeaveRange`
  (params (Target :type "MassEnemyTarget Structure"))
  (goto _label))

(event `self.OnAcquireNewTarget`
  (params (Target :type "MassEnemyTarget Structure")))

(event `self.OnTargetDeath`
  (goto _label))

(event `self.LoseSightOfTarget`)

(fn `CheckTargetVisible`
  (params (Target :type "MassEnemyTarget Structure"))
  (returns (ReturnValue :type Boolean))
  (bind _returnvalue (subsystem `EnemyManagerSubsystem`))
  (bind _outhit (`KismetSystemLibrary.LineTraceSingle` (`SceneComponent.K2_GetComponentLocation` (`self.Body`)) (`.Position` (break `MassEnemyTarget` Target)) "TraceTypeQuery1"))
  (bind (_outtarget _returnvalue_2) (`EnemyManagerSubsystem.GetEnemyTargetFromHit` _returnvalue _outhit))
  (return (and _returnvalue_2 (`EnemyManagerSubsystem.IsSameTarget` _returnvalue _outtarget Target))))

(fn `FireLaser`
  (locals (HitEnemies :type "Array of MassEnemyTarget Structure") (isSameTarget :type Boolean))
  (bind _returnvalue (`SceneComponent.K2_GetComponentLocation` (`self.Scene`)))
  (bind _outhits (`KismetSystemLibrary.SphereTraceMulti` :`Start` _returnvalue :`End` (+ (* (`SceneComponent.GetForwardVector` (`self.Body`)) (`KismetMathLibrary.Conv_IntToDouble` (`.Range` (break `TowerData` (`self.TowerData`))))) _returnvalue) :`Radius` 10.0 :`TraceChannel` "TraceTypeQuery5" :`DrawDebugType` "ForDuration" :`DrawTime` 1.0))
  ; Add to array if not already inside
  (for _array_element _outhits
    (bind (_outtarget _returnvalue_2) (`EnemyManagerSubsystem.GetEnemyTargetFromHit` (subsystem `EnemyManagerSubsystem`) _array_element))
    (if _returnvalue_2
      (set `local.isSameTarget` false)
      (for _array_element_2 (`local.HitEnemies`)
        (if (`EnemyManagerSubsystem.IsSameTarget` (subsystem `EnemyManagerSubsystem`) _array_element_2 _outtarget)
          (set `local.isSameTarget` true)
          (break)))
      (if (not (`local.isSameTarget`))
        (`KismetArrayLibrary.Array_Add` (`local.HitEnemies`) _outtarget))))
  (for _array_element_3 (`local.HitEnemies`)
    (if (`EnemyManagerSubsystem.IsTargetValid` (subsystem `EnemyManagerSubsystem`) _array_element_3)
      (bind _returnvalue_3 (`self.GetStats` (struct :`TagName` "Tower.Damage.BaseDamage")))
      (`EnemyManagerSubsystem.ApplyDamageToTarget` (subsystem `EnemyManagerSubsystem`) _array_element_3 (`KismetMathLibrary.FTrunc` _returnvalue_3)))))

(fn `UserConstructionScript`)