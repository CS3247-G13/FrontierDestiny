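; BP_Striker is a tower that fires a piercing laser along its barrel at enemies within range.
; It selects targets on activation, range entry and after each shot, slerping Joint yaw and Body pitch toward the target every tick.
; A looping cooldown triggers FireLaser, whose debug-drawn multi-sphere trace collects enemies to receive base damage and stat-driven damage over time.
; A line-trace helper checks target visibility.
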(event `self.OnTowerActive`
  (bind _cooldown (`self.Cooldown`))
  (`|ExecutionSequence`
    (:`then_0`
      ; Start cooldown
      (set `CooldownComponent.CooldownDuration` (`.Cooldown` (break `TowerData` (`self.TowerData`))) _cooldown)
      (`CooldownComponent.StartCooldown` _cooldown)
      (set `CooldownComponent.Mode` "LoopOnFinish" _cooldown))
    (:`then_1`
      (add `CooldownComponent.OnCooldownFinished` (`self.Cooldown`) (delegate `OnCooldownFinished_Event`)))
    (:`then_2`
      (`/Engine/EditorBlueprintResources/StandardMacros.IsValid` (`self.CurrentTarget`)
        (:`Is Not Valid`
          (`self.SelectTarget`))))))

(event `self.OnTowerTick`
  (params (DeltaTime :type "Float (single-precision)"))
  (`/Engine/EditorBlueprintResources/StandardMacros.IsValid` (`self.CurrentTarget`)
    (:`Is Valid`
      ; Rotate
      (`SceneComponent.K2_SetWorldRotation` (`self.Joint`) (`KismetMathLibrary.MakeRotator` 0.0 0.0 (.yaw (`TowerUtilities.QuaternionSlerp` (`KismetMathLibrary.MakeRotator` 0.0 (.pitch (`SceneComponent.RelativeRotation` (`self.Body`))) (.yaw (`SceneComponent.K2_GetComponentRotation` (`self.Joint`)))) (`KismetMathLibrary.MakeRotFromX` (`KismetMathLibrary.GetDirectionUnitVector` (`SceneComponent.K2_GetComponentLocation` (`self.Body`)) (`self.K2_GetActorLocation` (`self.CurrentTarget`)))) DeltaTime (`self.RotationSpeed`)))) false false)
      (`SceneComponent.K2_SetRelativeRotation` (`self.Body`) (`KismetMathLibrary.MakeRotator` 0.0 (.pitch (`TowerUtilities.QuaternionSlerp` (`KismetMathLibrary.MakeRotator` 0.0 (.pitch (`SceneComponent.RelativeRotation` (`self.Body`))) (.yaw (`SceneComponent.K2_GetComponentRotation` (`self.Joint`)))) (`KismetMathLibrary.MakeRotFromX` (`KismetMathLibrary.GetDirectionUnitVector` (`SceneComponent.K2_GetComponentLocation` (`self.Body`)) (`self.K2_GetActorLocation` (`self.CurrentTarget`)))) DeltaTime (`self.RotationSpeed`)))) false false))))

(event `OnCooldownFinished_Event`
  (`/Engine/EditorBlueprintResources/StandardMacros.IsValid` (`self.CurrentTarget`)
    (:`Is Valid`
      (`self.FireLaser`)
      (`self.SelectTarget`))))

(event `self.OnTargetEnterRange`
  (params (Target :type "Actor Object Reference"))
  (`self.SelectTarget`))

(fn `CheckTargetVisible`
  (params (Target :type "BaseEnemyCharacter Object Reference"))
  (returns (ReturnValue :type Boolean))
  (bind _outhit (`KismetSystemLibrary.LineTraceSingle` (`SceneComponent.K2_GetComponentLocation` (`self.Body`)) (`self.K2_GetActorLocation` Target) "TraceTypeQuery1"))
  (bind (_bblockinghit _binitialoverlap _time _distance _location _impactpoint _normal _impactnormal _physmat _hitactor) (`GameplayStatics.BreakHitResult` _outhit))
  (return (and (== _hitactor Target) _bblockinghit)))

(fn `FireLaser`
  (locals (`Hit Enemies` :type "Set of Actor Object Reference"))
  (bind _returnvalue (`SceneComponent.K2_GetComponentLocation` (`self.Scene`)))
  (bind _outhits (`KismetSystemLibrary.SphereTraceMulti` :`Start` _returnvalue :`End` (+ (* (`SceneComponent.GetForwardVector` (`self.Body`)) (`KismetMathLibrary.Conv_IntToDouble` (`.Range` (break `TowerData` (`self.TowerData`))))) _returnvalue) :`Radius` 10.0 :`TraceChannel` "TraceTypeQuery5" :`DrawDebugType` "ForDuration" :`DrawTime` 1.0))
  (for _array_element _outhits
    (bind _asbase_enemy_character (cast `BaseEnemyCharacter` (`.HitActor` (`GameplayStatics.BreakHitResult` _array_element))))
    (`BlueprintSetLibrary.Set_Add` (`local.Hit Enemies`) _asbase_enemy_character))
  (bind _valuepin (`|SetForEach` (`local.Hit Enemies`))
    (:`then`
      (`/Engine/EditorBlueprintResources/StandardMacros.IsValid` _valuepin
        (:`Is Valid`
          (`|ExecutionSequence`
            (:`then_0`
              (bind _returnvalue_2 (`self.GetComponentByClass` _valuepin "/Script/FrontierDestiny.StatusEffectComponent"))
              (`/Engine/EditorBlueprintResources/StandardMacros.IsValid` _returnvalue_2
                (:`Is Valid`
                  (bind _returnvalue_3 (`self.GetStats` (struct :`TagName` "Tower.Damage.DOT")))
                  (bind _returnvalue_4 (`self.GetStats` (struct :`TagName` "Tower.Damage.DOT.Duration")))
                  (`StatusEffectComponent.ApplyDOTByDamagePerSecond` _returnvalue_2 "Pewpew" _returnvalue_3 _returnvalue_4 1.0 (`self.GetInstigatorController`) self))))
            (:`then_1`
              (`GameplayStatics.ApplyDamage` _valuepin (`.Amount` (break `TowerEffect` (`BlueprintMapLibrary.Map_Find` (`.Effects` (break `TowerData` (`self.TowerData`))) (struct :`TagName` "Tower.Damage.BaseDamage")))) (`self.GetInstigatorController`) self))))))))

(fn `UserConstructionScript`)