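; BP_ArcTrap is a single-use arc trap tower that damages and stuns enemies around it when its proximity trigger fires.
; A DoOnce-guarded trigger event runs a sphere trace sized by the AOE radius stat, deduplicates the enemy targets, then destroys the tower.
; Each target receives stat-driven Electric damage and a stun through the EnemyManagerSubsystem.
; The arc lightning effect call is disconnected and never runs.
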(event `self.OnProximityTriggered`
  (params (Target :type "MassEnemyTarget Structure"))
  (bind _returnvalue (`SceneComponent.K2_GetComponentLocation` (`self.RangeComponent`)))
  (`/Engine/EditorBlueprintResources/StandardMacros.DoOnce` false
    (:`Completed`
      (bind _outhits (`KismetSystemLibrary.SphereTraceMulti` _returnvalue _returnvalue (`self.GetStats` (struct :`TagName` "Tower.Damage.AOE.Radius")) "TraceTypeQuery5"))
      (bind _returnvalue_2 (`TowerBlueprintFunctionLibrary.GetUniqueEnemyTargetsFromHits` _outhits (`|MakeArray` (struct) :!type "MassEnemyTarget Structure")))
      (for _array_element _returnvalue_2
        (`self.DamageEnemy` _array_element))
      (`self.DestroyTower`))))

(fn `DamageEnemy`
  (params (Target :type "MassEnemyTarget Structure"))
  (bind _returnvalue (subsystem `EnemyManagerSubsystem`))
  (`EnemyManagerSubsystem.ApplyDamageToTarget` _returnvalue Target (`KismetMathLibrary.FTrunc` (`self.GetStats` (struct :`TagName` "Tower.Damage.BaseDamage"))) (`.Position` (break `MassEnemyTarget` Target)) "Electric")
  (`EnemyManagerSubsystem.ApplyStun` _returnvalue Target (`self.GetStats` (struct :`TagName` "Tower.Utility.StunDuration"))))

(fn `UserConstructionScript`)