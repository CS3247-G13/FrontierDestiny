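; BP_BlazeTrap is a tower trap that sets the enemies it damages on fire.
; It overrides DamageEnemy, running the parent damage logic and then asking the enemy manager subsystem to apply a burn to the target.
; Burn duration, damage per tick and tick interval come from the tower's tag-keyed DOT stats.
; All other behavior is inherited, as its event graph holds only disabled stubs.
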(fn `DamageEnemy`
  (params (Target :type "MassEnemyTarget Structure"))
  (`parent.DamageEnemy` Target)
  (`EnemyManagerSubsystem.ApplyBurn` (subsystem `EnemyManagerSubsystem`) Target (`self.GetStats` (struct :`TagName` "Tower.Damage.DOT.Duration")) (`self.GetStats` (struct :`TagName` "Tower.Damage.DOT.DamagePerTick")) (`self.GetStats` (struct :`TagName` "Tower.Damage.DOT.TickInterval"))))

(fn `UserConstructionScript`
  (`parent.UserConstructionScript`))