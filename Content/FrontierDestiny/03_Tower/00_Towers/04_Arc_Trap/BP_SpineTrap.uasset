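; BP_SpineTrap is a proximity-triggered trap tower that fires a burst of spines.
; It overrides the proximity trigger to spawn a Niagara burst, sized by the tower's AOE damage radius stat, and play a spines sound at its location.
; It then calls the parent trigger, which holds any further behavior; MakeEmitter is an empty stub.
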(event `self.OnProximityTriggered`
  (params (Target :type "MassEnemyTarget Structure"))
  (bind _returnvalue (`SceneComponent.K2_GetComponentLocation` (`self.RootComponent`)))
  (bind _returnvalue_2 (`NiagaraFunctionLibrary.SpawnSystemAtLocation` "/Game/FrontierDestiny/Levels/ParticleEffects/NS_SpineBurst.NS_SpineBurst" _returnvalue))
  (`NiagaraComponent.SetVariableFloat` _returnvalue_2 "Radius" (`self.GetStats` (struct :`TagName` "Tower.Damage.AOE.Radius")))
  (`GameplayStatics.PlaySoundAtLocation` "/Game/FrontierDestiny/03_Tower/Audio/SpineTrap_Spines.SpineTrap_Spines" _returnvalue (struct) 2.0 1.0 0.0 "/Game/FrontierDestiny/03_Tower/Audio/TowerAttenuation.TowerAttenuation" null null null)
  (`parent.OnProximityTriggered` (struct)))

(fn `MakeEmitter`
  (params (TargetLoc :type "Vector Structure") (Origin :type "Vector Structure"))
  (return))

(fn `UserConstructionScript`
  (`parent.UserConstructionScript`))