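; BP_HeavenStorm is a tower Blueprint in the God Rod family that adds stun and an electric projectile to its inherited attack.
; Main and peripheral damage overrides run the parent logic, then stun the target through the enemy manager subsystem, using the tower's StunDuration stat.
; The MakeProjectile override spawns a BP_ElectricMetalChunk with the given radius, owner and direction at zero initial speed, and prints a debug string.
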(fn `DamageMainEnemy`
  (params (Target :type "MassEnemyTarget Structure") (`Impact Location` :type "Vector Structure"))
  (`parent.DamageMainEnemy` Target `Impact Location`)
  (`EnemyManagerSubsystem.ApplyStun` (subsystem `EnemyManagerSubsystem`) Target (`self.GetStats` (struct :`TagName` "Tower.Utility.StunDuration"))))

(fn `DamagePeripheralEnemy`
  (params (Target :type "MassEnemyTarget Structure") (`Impact Location` :type "Vector Structure"))
  (`parent.DamagePeripheralEnemy` Target `Impact Location`)
  (`EnemyManagerSubsystem.ApplyStun` (subsystem `EnemyManagerSubsystem`) Target (`self.GetStats` (struct :`TagName` "Tower.Utility.StunDuration"))))

(fn `MakeProjectile`
  (params (Transform :type "Transform Structure") (Radius :type "Float (double-precision)") (Owner :type "/Game/FrontierDestiny/03_Tower/00_Towers/00_God_Rod/BP_God_Rod Object Reference") (Direction :type "Vector Structure") (Instigator :type "Pawn Object Reference"))
  (returns (Proj :type "/Game/FrontierDestiny/03_Tower/00_Towers/00_God_Rod/Rock/BP_DenseMetalChunk Object Reference"))
  (bind _returnvalue (`|SpawnActorFromClass` "/Game/FrontierDestiny/03_Tower/00_Towers/00_God_Rod/Rock/BP_ElectricMetalChunk.BP_ElectricMetalChunk_C" Transform "Undefined" "MultiplyWithRoot" null 100.0 Radius true Owner Direction 0.0 Instigator))
  (`KismetSystemLibrary.PrintString` "HeavenStorm Projectile Spawning")
  (return _returnvalue))

(fn `UserConstructionScript`
  (`parent.UserConstructionScript`))