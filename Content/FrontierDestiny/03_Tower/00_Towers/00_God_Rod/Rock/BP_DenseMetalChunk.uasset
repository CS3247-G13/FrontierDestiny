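; Dense metal chunk projectile of the God Rod tower that spins and deals kinetic impact damage to enemies.
; When it hits while not charging, the owning tower damages the struck target, then unique peripheral targets found by a sphere trace via the enemy manager.
; Impact also draws a debug radius sphere and spawns a Niagara blast before calling the parent hit logic.
; Spin speed scales with actor size, and lifespan is set at BeginPlay.
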(event `self.HitTarget`
  (params (Hit :type "HitResult Structure (by ref)"))
  (bind (_bblockinghit _binitialoverlap _time _distance _location _impactpoint) (`GameplayStatics.BreakHitResult` Hit))
  (bind _radius (`self.Radius`))
  (bind (_outtarget _returnvalue) (`EnemyManagerSubsystem.GetEnemyTargetFromHit` (subsystem `EnemyManagerSubsystem`) Hit))
  (if (not (`self.Charging`))
    (`|ExecutionSequence`
      (:`then_0`
        (if _returnvalue
          ; Damage Main Enemy
          (`/Game/FrontierDestiny/03_Tower/00_Towers/00_God_Rod/BP_God_Rod.DamageMainEnemy` (`self.Tower Owner`) _outtarget (`.ImpactPoint` (`GameplayStatics.BreakHitResult` Hit)))))
      (:`then_1`
        ; Do AOE damage
        (bind _outhits (`KismetSystemLibrary.SphereTraceMulti` _impactpoint _impactpoint _radius "TraceTypeQuery5"))
        (bind _returnvalue_2 (`TowerBlueprintFunctionLibrary.GetUniqueEnemyTargetsFromHits` _outhits (select `bool` (`EnemyManagerSubsystem.IsTargetValid` (subsystem `EnemyManagerSubsystem`) _outtarget) :`true` (`|MakeArray` _outtarget))))
        (for _array_element _returnvalue_2
          (`/Game/FrontierDestiny/03_Tower/00_Towers/00_God_Rod/BP_God_Rod.DamagePeripheralEnemy` (`self.Tower Owner`) _array_element (`.Position` (break `MassEnemyTarget` _array_element)))))
      (:`then_2`
        (`KismetSystemLibrary.DrawDebugSphere` _impactpoint _radius 12 (struct :`R` 1.0 :`G` 0.046449 :`A` 1.0) 5.0 1.0)
        (`NiagaraFunctionLibrary.SpawnSystemAtLocation` "/Game/FrontierDestiny/Levels/ParticleEffects/NS_KineticBlast.NS_KineticBlast" (`self.K2_GetActorLocation`)))
      (:`then_3`
        (`parent.HitTarget` Hit)))))

(event `self.ReceiveBeginPlay`
  (`self.SetLifeSpan` (`self.Lifespan`)))

(event `self.ReceiveTick`
  (params (DeltaSeconds :type "Float (single-precision)"))
  (`SceneComponent.K2_AddWorldRotation` (`self.rock1`) (`KismetMathLibrary.MakeRotator` (.x (* (`KismetMathLibrary.VSize` (`self.GetActorScale3D`)) DeltaSeconds (`KismetMathLibrary.MakeVector` (.roll (`self.Rotation`)) (.pitch (`self.Rotation`)) (.yaw (`self.Rotation`))))) (.y (* (`KismetMathLibrary.VSize` (`self.GetActorScale3D`)) DeltaSeconds (`KismetMathLibrary.MakeVector` (.roll (`self.Rotation`)) (.pitch (`self.Rotation`)) (.yaw (`self.Rotation`))))) (.z (* (`KismetMathLibrary.VSize` (`self.GetActorScale3D`)) DeltaSeconds (`KismetMathLibrary.MakeVector` (.roll (`self.Rotation`)) (.pitch (`self.Rotation`)) (.yaw (`self.Rotation`)))))) false false))

(fn `UserConstructionScript`)