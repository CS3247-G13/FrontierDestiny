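; God Rod tower that charges and fires a dense metal chunk projectile with direct and area damage, tuned by tagged TowerData effects.
; It slerps joint yaw and head pitch toward its target, using a Visibility trace for line-of-sight checks.
; Cooldown completion spawns a zero-scale chunk attached to the head, which grows with cooldown progress.
; Once grow time passes, the chunk detaches and launches forward, and the tower reselects a target shortly after.
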(event `self.OnTowerTick`
  (params (DeltaTime :type "Float (single-precision)"))
  (bind _currentbullet (`self.CurrentBullet`))
  (bind _currentbullet_2 (`self.CurrentBullet`))
  (bind _cooldown (`self.Cooldown`))
  (bind _returnvalue (`CooldownComponent.GetProgressPercent` (`self.Cooldown`)))
  (bind _returnvalue_2 (/ (`.Amount` (break `TowerEffect` (`BlueprintMapLibrary.Map_Find` (`.Effects` (break `TowerData` (`self.TowerData`))) (struct :`TagName` "Tower.GodRod.Projectile.GrowTime")))) (`.Cooldown` (break `TowerData` (`self.TowerData`)))))
  (`|ExecutionSequence`
    (:`then_0`
      (`/Engine/EditorBlueprintResources/StandardMacros.IsValid` (`self.CurrentTarget`)
        (:`Is Not Valid`
          (`self.SelectTarget`))))
    (:`then_1`
      (`/Engine/EditorBlueprintResources/StandardMacros.IsValid` (`self.CurrentTarget`)
        (:`Is Valid`
          (`|ExecutionSequence`
            (:`then_0`
              (`SceneComponent.K2_SetWorldRotation` (`self.Tower_Joint`) (`KismetMathLibrary.MakeRotator` 0.0 0.0 (.yaw (`TowerUtilities.QuaternionSlerp` (`KismetMathLibrary.MakeRotator` 0.0 (.pitch (`SceneComponent.RelativeRotation` (`self.TowerHead`))) (.yaw (`SceneComponent.K2_GetComponentRotation` (`self.Tower_Joint`)))) (`KismetMathLibrary.MakeRotFromX` (`KismetMathLibrary.GetDirectionUnitVector` (`SceneComponent.K2_GetComponentLocation` (`self.TowerHead`)) (`self.K2_GetActorLocation` (`self.CurrentTarget`)))) DeltaTime (`.Amount` (break `TowerEffect` (`BlueprintMapLibrary.Map_Find` (`.Effects` (break `TowerData` (`self.TowerData`))) (struct :`TagName` "Tower.Movement.RotationSpeed"))))))) false false)
              (`SceneComponent.K2_SetRelativeRotation` (`self.TowerHead`) (`KismetMathLibrary.MakeRotator` 0.0 (.pitch (`TowerUtilities.QuaternionSlerp` (`KismetMathLibrary.MakeRotator` 0.0 (.pitch (`SceneComponent.RelativeRotation` (`self.TowerHead`))) (.yaw (`SceneComponent.K2_GetComponentRotation` (`self.Tower_Joint`)))) (`KismetMathLibrary.MakeRotFromX` (`KismetMathLibrary.GetDirectionUnitVector` (`SceneComponent.K2_GetComponentLocation` (`self.TowerHead`)) (`self.K2_GetActorLocation` (`self.CurrentTarget`)))) DeltaTime (`.Amount` (break `TowerEffect` (`BlueprintMapLibrary.Map_Find` (`.Effects` (break `TowerData` (`self.TowerData`))) (struct :`TagName` "Tower.Movement.RotationSpeed"))))))) false false))
            (:`then_1`
              (`/Engine/EditorBlueprintResources/StandardMacros.DoOnce` false
                (:`Completed`
                  (`self.OnCooldownFinished_Event`)
                  (`CooldownComponent.ResetCooldown` _cooldown)
                  (`CooldownComponent.StartCooldown` _cooldown))))))))
    (:`then_2`
      ; Scale the bullet
      (`/Engine/EditorBlueprintResources/StandardMacros.IsValid` _currentbullet
        (:`Is Valid`
          (`SceneComponent.SetWorldScale3D` (`/Game/FrontierDestiny/03_Tower/00_Towers/00_God_Rod/Rock/BP_DenseMetalChunk.rock` _currentbullet) (`KismetMathLibrary.Conv_DoubleToVector` (* (/ _returnvalue _returnvalue_2) (`.Amount` (break `TowerEffect` (`BlueprintMapLibrary.Map_Find` (`.Effects` (break `TowerData` (`self.TowerData`))) (struct :`TagName` "Tower.GodRod.Projectile.MaxSize")))))))
          (if (> _returnvalue _returnvalue_2)
            ; Launch
            (set `StraightProjectileActor.Speed` (`self.ProjectileSpeed`) _currentbullet_2)
            (set `StraightProjectileActor.Direction` (`SceneComponent.GetForwardVector` (`self.TowerHead`)) _currentbullet_2)
            (set `/Game/FrontierDestiny/03_Tower/00_Towers/00_God_Rod/Rock/BP_DenseMetalChunk.Charging` false _currentbullet_2)
            (`self.K2_DetachFromActor` _currentbullet_2 "KeepWorld" "KeepWorld" "KeepWorld")
            (set `self.CurrentBullet` null)
            (`KismetSystemLibrary.Delay` 0.5)
            (`self.SelectTarget`)))))))

(event `self.OnTowerActive`
  (bind _cooldown (`self.Cooldown`))
  ; Setup
  (set `CooldownComponent.CooldownDuration` (`.Cooldown` (break `TowerData` (`self.TowerData`))) _cooldown)
  (`CooldownComponent.StartCooldown` _cooldown)
  (add `CooldownComponent.OnCooldownFinished` _cooldown (delegate `OnCooldownFinished_Event`)))

(event `OnCooldownFinished_Event`
  (bind _cooldown (`self.Cooldown`))
  ; Setup
  (`/Engine/EditorBlueprintResources/StandardMacros.IsValid` (`self.CurrentTarget`)
    (:`Is Valid`
      (`CooldownComponent.ResetCooldown` _cooldown)
      (`CooldownComponent.StartCooldown` _cooldown)
      (`self.SpawnBullet`))))

(event `self.ReceiveEndPlay`
  (params (EndPlayReason :type "EEndPlayReason Enum" :default "Destroyed"))
  (bind _currentbullet (`self.CurrentBullet`))
  (`/Engine/EditorBlueprintResources/StandardMacros.IsValid` _currentbullet
    (:`Is Valid`
      (`self.K2_DestroyActor` _currentbullet))))

(event `self.OnTargetEnterRange`
  (params (Target :type "Actor Object Reference"))
  (`self.SelectTarget`))

(fn `CheckTargetVisible`
  (params (Target :type "BaseEnemyCharacter Object Reference"))
  (returns (ReturnValue :type Boolean))
  (bind _currentbullet (`self.CurrentBullet`))
  (bind _outhit (`KismetSystemLibrary.LineTraceSingle` (`SceneComponent.K2_GetComponentLocation` (`self.TowerHead`)) (`self.K2_GetActorLocation` Target) "TraceTypeQuery1" false (select `bool` (`KismetSystemLibrary.IsValid` _currentbullet) :`true` (`|MakeArray` _currentbullet :!type "Actor Object Reference"))))
  (bind (_bblockinghit _binitialoverlap _time _distance _location _impactpoint _normal _impactnormal _physmat _hitactor) (`GameplayStatics.BreakHitResult` _outhit))
  (return (and (== _hitactor Target) _bblockinghit)))

(fn `SpawnBullet`
  (bind (_class _cost _name _description _icon _range _health _cooldown _footprint _boundary _pivotpoint _height _effects) (break `TowerData` (`self.TowerData`)))
  (bind _returnvalue (`|SpawnActorFromClass` "/Game/FrontierDestiny/03_Tower/00_Towers/00_God_Rod/Rock/BP_DenseMetalChunk.BP_DenseMetalChunk_C" (`KismetMathLibrary.MakeTransform` (.location (`SceneComponent.K2_GetComponentToWorld` (`self.Spawner`))) (.rotation (`SceneComponent.K2_GetComponentToWorld` (`self.Spawner`))) (0.0 0.0 0.0)) "Undefined" "MultiplyWithRoot" null (`.Amount` (break `TowerEffect` (`BlueprintMapLibrary.Map_Find` _effects (struct :`TagName` "Tower.Damage.AOE.BaseDamage")))) (`.Amount` (break `TowerEffect` (`BlueprintMapLibrary.Map_Find` _effects (struct :`TagName` "Tower.Damage.BaseDamage")))) 100.0 (`.Amount` (break `TowerEffect` (`BlueprintMapLibrary.Map_Find` _effects (struct :`TagName` "Tower.Damage.AOE.Radius")))) true (`SceneComponent.GetForwardVector` (`self.TowerHead`)) 0.0 (`self.GetInstigator`)))
  (set `self.CurrentBullet` _returnvalue)
  (`self.K2_AttachToComponent` _returnvalue (`self.TowerHead`) "None" "KeepWorld" "KeepRelative" "KeepRelative" true))

(fn `UserConstructionScript`)