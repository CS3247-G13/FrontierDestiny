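; BP_Cutscener is an actor that triggers a showcase cutscene tied to quest progress.
; On BeginPlay it binds to the quest subsystem's quest-updated event.
; When the current quest is Horde_4, it waits through a delay, confirms the player controller is a TowerDemoPlayerController, then creates a level sequence player and plays LS_ShowcaseCores.
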(event `self.ReceiveBeginPlay`
  (add `QuestSubsystem.OnQuestUpdated` (subsystem `QuestSubsystem`) (delegate `On Quest Updated`)))

(event `On Quest Updated`
  (if (== (`.QuestID` (break `QuestData` (`QuestSubsystem.CurrentQuest` (subsystem `QuestSubsystem`)))) "Horde_4")
    (`KismetSystemLibrary.Delay` 9.0)
    (cast `TowerDemoPlayerController` (`GameplayStatics.GetPlayerController` 0))
    (bind (_outactor _returnvalue) (`LevelSequencePlayer.CreateLevelSequencePlayer` "/Game/FrontierDestiny/97_Cutscenes/LS_ShowcaseCores.LS_ShowcaseCores"))
    (`MovieSceneSequencePlayer.Play` _returnvalue)))

(fn `UserConstructionScript`)