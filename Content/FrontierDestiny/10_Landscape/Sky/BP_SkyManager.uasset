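; BP_SkyManager blends the GoodSky sky actor toward a biome preset.
; SetBiome stores the target preset, snapshots current sky values and restarts a blend timeline.
; Each timeline update lerps the global overlay color and custom-mode time of day, then calls GoodSky's realtime update.
; Cloud coverage and sky effect are captured but never blended or applied.
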(event `Set Biome`
  (params (TargetPreset :type "/Game/FrontierDestiny/10_Landscape/Sky/DA_SkyPreset Object Reference"))
  (bind _goodskyref (`self.GoodSkyRef`))
  (bind _goodskyref_2 (`self.GoodSkyRef`))
  (set `self.TargetPreset` TargetPreset)
  (set `self.└ Time of Day ( For Custom Mode )` (`/Game/GoodSky/Blueprint/BP_MasterGoodSky.└ Time of Day ( For Custom Mode )` _goodskyref))
  (set `self.Sky Clouds Coverage Preset` (`/Game/GoodSky/Blueprint/BP_MasterGoodSky.SkyCloudsCoveragePreset` _goodskyref))
  (set `self.Sky Effect` (`/Game/GoodSky/Blueprint/BP_MasterGoodSky.SkyEffect` _goodskyref))
  (set `self.Global Overlay Color` (`/Game/GoodSky/Blueprint/BP_MasterGoodSky.Global Overlay Color` _goodskyref))
  (bind (_direction _alpha) (`Timeline|BlendTimeline` :!via `PlayFromStart`)
    (:`Update`
      (set `/Game/GoodSky/Blueprint/BP_MasterGoodSky.Global Overlay Color` (`KismetMathLibrary.LinearColorLerp` (`self.Global Overlay Color`) (`/Game/FrontierDestiny/10_Landscape/Sky/DA_SkyPreset.Global Overlay Color` (`self.TargetPreset`)) _alpha) _goodskyref_2)
      (set `/Game/GoodSky/Blueprint/BP_MasterGoodSky.└ Time of Day ( For Custom Mode )` (`KismetMathLibrary.Lerp` (`self.└ Time of Day ( For Custom Mode )`) (`/Game/FrontierDestiny/10_Landscape/Sky/DA_SkyPreset.└ Time of Day ( For Custom Mode )` (`self.TargetPreset`)) _alpha) _goodskyref_2)
      (`/Game/GoodSky/Blueprint/BP_MasterGoodSky.GoodSky Realtime Update` _goodskyref_2))))

(fn `UserConstructionScript`)