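; Shootable sea mine that explodes after enough hits on its mine mesh, dealing area damage to enemies, then regrows.
; Each hit removes one health and tints a dynamic material toward a damaged color; health fully resets after a cooldown without hits.
; At zero it spawns a Niagara blast and sound, damages sphere-traced targets through the enemy manager subsystem, then scales up from zero until re-armed.
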(event `Enable Mine`
  ;[1 1 1] Enable the mine and set health
  (set `self.Enabled` true)
  (set `self.Current Health` (`self.Max Health`))
  (`MaterialInstanceDynamic.SetVectorParameterValue` (`self.MID`) "BaseColorFactor" (struct :`R` 1.0 :`G` 1.0 :`B` 1.0 :`A` 1.0))
  (bind _output_get (set `self.Regeneration Progress` 1.0))
  (`SceneComponent.SetRelativeScale3D` (`self.mine`) (`KismetMathLibrary.Conv_DoubleToVector` _output_get)))

(event `self.ReceiveTick`
  (params (DeltaSeconds :type "Float (single-precision)"))
  (if (`self.Enabled`)
    ; If not disabled, tick down the heal cooldown
    (bind _output_get (set `self.Remaining Heal Cooldown` (`KismetMathLibrary.FMax` (- (`self.Remaining Heal Cooldown`) DeltaSeconds))))
    (if (== _output_get 0.0)
      (set `self.Current Health` (`self.Max Health`))
      (`self.On Health Change`))
    (else
      ;[0 0 0] If disabled, grow the mine back
      (bind _output_get_2 (set `self.Regeneration Progress` (`KismetMathLibrary.FMin` (+ (`self.Regeneration Progress`) (* DeltaSeconds (/ 1.0 (`self.Rearm Cooldown`)))) 1.0)))
      (`SceneComponent.SetRelativeScale3D` (`self.mine`) (`KismetMathLibrary.Conv_DoubleToVector` _output_get_2))
      (if (== _output_get_2 1.0)
        (`self.Enable Mine`)))))

(event `self.ReceiveBeginPlay`
  ; INITIALIZE MATERIAL
  (`|ExecutionSequence`
    (:`then_0`
      (bind _returnvalue (`KismetMaterialLibrary.CreateDynamicMaterialInstance` (`PrimitiveComponent.GetMaterial` (`self.mine`) 0)))
      (bind _output_get (set `self.MID` _returnvalue))
      (`MaterialInstanceDynamic.SetVectorParameterValue` _output_get "BaseColorFactor" (struct :`R` 1.0 :`G` 1.0 :`B` 1.0 :`A` 1.0))
      (`PrimitiveComponent.SetMaterial` (`self.mine`) 0 _output_get))
    (:`then_1`
      (`self.Enable Mine`))))

(event `Explode`
  (bind _returnvalue (`SceneComponent.K2_GetComponentLocation` (`self.mine`)))
  ;[0.15 0.008885 3.3e-05] Explode the mine
  (set `self.Regeneration Progress` 0.0)
  (set `self.Enabled` false)
  (`MaterialInstanceDynamic.SetVectorParameterValue` (`self.MID`) "BaseColorFactor" (`self.Growing Color`))
  (bind _returnvalue_2 (`NiagaraFunctionLibrary.SpawnSystemAtLocation` "/Game/FrontierDestiny/Levels/ParticleEffects/NS_KineticBlast.NS_KineticBlast" _returnvalue))
  (`FXSystemComponent.SetFloatParameter` _returnvalue_2 "Radius" (`self.Radius`))
  (`GameplayStatics.PlaySoundAtLocation` (`self.Explosion Sound`) _returnvalue (struct) 1.0 1.0 0.0 null null null null)
  ; Do AOE damage
  (bind _outhits (`KismetSystemLibrary.SphereTraceMulti` _returnvalue _returnvalue (`self.Radius`) "TraceTypeQuery5"))
  (bind _returnvalue_3 (`TowerBlueprintFunctionLibrary.GetUniqueEnemyTargetsFromHits` _outhits (`|MakeArray` (struct) :!type "MassEnemyTarget Structure")))
  (for _array_element _returnvalue_3
    (`EnemyManagerSubsystem.ApplyDamageToTarget` (subsystem `EnemyManagerSubsystem`) _array_element (`self.Damage`) (`.Position` (break `MassEnemyTarget` _array_element)) (`self.Damage Type`))))

(event `self.Shoot`
  (params (Hit :type "HitResult Structure (by ref)") (Damage :type Integer))
  (if (and (`self.Enabled`) (== (`.HitComponent` (`GameplayStatics.BreakHitResult` Hit)) (`self.mine`)))
    ;[0.15 0.01828 0.005369 0.5] REDUCE CURRENT HEALTH BY 1 (CAN CHANGE TO USE THE DAMAGE)
    (bind _output_get (set `self.Current Health` (`KismetMathLibrary.Max` (- (`self.Current Health`) 1))))
    ; Reset the heal cooldown
    (set `self.Remaining Heal Cooldown` (`self.Heal Cooldown`))
    ; Explode if no more health
    (if (== _output_get 0)
      (`self.Explode`)
      (else
        (`self.On Health Change`)))))

(event `On Health Change`
  (bind _returnvalue (/ (`KismetMathLibrary.Conv_IntToDouble` (`self.Current Health`)) (`self.Max Health`)))
  ; IF STILL HAVE HEALTH. UPDATE COLOR TO INDICATE DAMAGE
  (`MaterialInstanceDynamic.SetVectorParameterValue` (`self.MID`) "BaseColorFactor" (+ (* (`self.Damaged Color`) (- 1.0 _returnvalue)) (* _returnvalue (`self.Default Color`)))))

(fn `UserConstructionScript`)