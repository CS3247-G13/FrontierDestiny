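; Mass spawner Blueprint that runs a timed wave of enemy spawns when play begins.
; Wave1 starts a looping two-second timer that calls DoSpawning and increments a counter, clearing itself once the maximum count is reached.
; A separate looping timer polls the quest subsystem for Quest_Four and, when it is current, only stops its own polling without starting another wave.
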(event `self.ReceiveBeginPlay`
  (`self.Wave1`)
  (bind _returnvalue (`KismetSystemLibrary.K2_SetTimerDelegate` (delegate `Check Event`) 2.0 true)))

(event `Check Event`
  (if (== (`.QuestID` (break `QuestData` (`QuestSubsystem.CurrentQuest` (subsystem `QuestSubsystem`)))) "Quest_Four")
    (`KismetSystemLibrary.K2_ClearAndInvalidateTimerHandle` (stale `self.ReceiveBeginPlay` _returnvalue))))

(event `Wave1`
  (bind _returnvalue (`KismetSystemLibrary.K2_SetTimerDelegate` (delegate `SpawnEnemy`) 2.0 true))
  (set `self.Current Timer` _returnvalue)
  (set `self.MaxSpawnCount` 10.0)
  (set `self.CurrentSpawnCount` 0.0))

(event `SpawnEnemy`
  (`/Engine/EditorBlueprintResources/StandardMacros.IncrementFloat` (`self.CurrentSpawnCount`)
    (:`  `
      (`self.DoSpawning`)
      (if (<= (`self.MaxSpawnCount`) (`self.CurrentSpawnCount`))
        (`KismetSystemLibrary.K2_ClearAndInvalidateTimerHandle` (`self.Current Timer`))))))

(fn `UserConstructionScript`)