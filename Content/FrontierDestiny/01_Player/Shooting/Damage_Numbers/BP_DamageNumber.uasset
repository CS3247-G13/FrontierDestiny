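; BP_DamageNumber is a world-space damage number actor that displays its Text value through a TextRender component.
; BeginPlay sets the rendered text once.
; Tick accumulates delta time in Progress and uses the clamped value for the text's X and Y scale, growing it to full size over about a second.
; The graph contains no movement, fade or destroy logic.
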(event `self.ReceiveBeginPlay`
  (`TextRenderComponent.K2_SetText` (`self.TextRender`) (`KismetTextLibrary.Conv_StringToText` (`self.Text`))))

(event `self.ReceiveTick`
  (params (DeltaSeconds :type "Float (single-precision)"))
  (bind _textrender (`self.TextRender`))
  (bind _returnvalue (+ (`self.Progress`) DeltaSeconds))
  (bind _returnvalue_2 (`KismetMathLibrary.FClamp` _returnvalue))
  (set `self.Progress` _returnvalue)
  (`TextRenderComponent.SetXScale` _textrender _returnvalue_2)
  (`TextRenderComponent.SetYScale` _textrender _returnvalue_2))

(fn `UserConstructionScript`)