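; Player Blueprint that wires up movement, combat, interaction and pausing.
; On BeginPlay it sets walk speed from the PlayerManagerSubsystem's PlayerData and hands shotgun and sniper muzzle flashes to the Combat component.
; Interact input calls the Interactor, while Pause toggles game pause along with the pause menu widget, input mode and mouse cursor.
; Incoming damage only prints a debug message, with no health handling here.
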(event `self.ReceiveBeginPlay`
  (set `CharacterMovementComponent.MaxWalkSpeed` (`.MovementSpeed` (break `PlayerData` (`PlayerManagerSubsystem.PlayerData` (subsystem `PlayerManagerSubsystem`)))) (`self.CharacterMovement`))
  (`CombatComponent.SetMuzzleFlashes` (`self.Combat`) (`self.P_Shotgun`) (`self.P_Sniper`)))

(event `self.ReceiveAnyDamage`
  (params (Damage :type "Float (single-precision)") (DamageType :type "DamageType Object Reference") (InstigatedBy :type "Controller Object Reference") (DamageCauser :type "Actor Object Reference"))
  (`KismetSystemLibrary.PrintString` (`KismetStringLibrary.Concat_StrStr` "Ouch. " (`KismetSystemLibrary.GetDisplayName` InstigatedBy) "Dealt " (`KismetStringLibrary.Conv_DoubleToString` Damage) " damage.")))

(event `EnhancedInput|/Game/FrontierDestiny/01_Player/Input/IA_Interact`
  (params (ActionValue :type Boolean) (ElapsedSeconds :type "Float (double-precision)") (TriggeredSeconds :type "Float (double-precision)") (InputAction :type "InputAction Object Reference" :default "/Game/FrontierDestiny/01_Player/Input/IA_Interact.IA_Interact"))
  ; Interact code is here because I am lazy
  (:`Triggered`
    (`KismetSystemLibrary.PrintString` "Hello")
    (`InteractorComponent.Interact` (`self.Interactor`))))

(event `EnhancedInput|/Game/FrontierDestiny/01_Player/Input/IA_Pause`
  (params (ActionValue :type Boolean) (ElapsedSeconds :type "Float (double-precision)") (TriggeredSeconds :type "Float (double-precision)") (InputAction :type "InputAction Object Reference" :default "/Game/FrontierDestiny/01_Player/Input/IA_Pause.IA_Pause"))
  (bind _returnvalue (`GameplayStatics.GetPlayerController` 0))
  (:`Started`
    (if (`GameplayStatics.IsGamePaused`)
      (`Widget.RemoveFromParent` (`self.PauseMenuRef`))
      (`WidgetBlueprintLibrary.SetInputMode_GameOnly` _returnvalue)
      (set `PlayerController.bShowMouseCursor` false _returnvalue)
      (`GameplayStatics.SetGamePaused` false)
      (else
        (bind _returnvalue_2 (`|CreateWidget` "/Game/FrontierDestiny/09_PauseMenu/WBP_PauseMenu.WBP_PauseMenu_C"))
        (bind _output_get (set `self.PauseMenuRef` _returnvalue_2))
        (`UserWidget.AddToViewport` _output_get 0)
        (`WidgetBlueprintLibrary.SetInputMode_GameAndUIEx` _returnvalue _output_get)
        (set `PlayerController.bShowMouseCursor` true _returnvalue)
        (`GameplayStatics.SetGamePaused` true)))))

(fn `UserConstructionScript`)