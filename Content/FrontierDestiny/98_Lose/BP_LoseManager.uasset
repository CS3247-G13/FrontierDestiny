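; Lose manager actor that runs the defeat sequence when the CoreManagerSubsystem reports a captured core destroyed.
; It plays that core's level sequence from an index-matched array, clears input mappings, and after a delay shows the lose widget, frees the mouse and pauses.
; Parallel to that delay, it plays the lose sound, spawns an explosion at the core, moves attached actors to world origin and destroys the core.
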(event `self.ReceiveBeginPlay`
  (add `CoreManagerSubsystem.OnCapturedCoreDestroyed` (subsystem `CoreManagerSubsystem`) (delegate `On Destroyed`)))

(event `On Destroyed`
  (params (CoreIndex :type Integer))
  (bind _returnvalue (`GameplayStatics.GetPlayerController` 0))
  (bind _returnvalue_2 (`CoreManagerSubsystem.GetCore` (subsystem `CoreManagerSubsystem`) CoreIndex))
  (`|ExecutionSequence`
    (:`then_0`
      (bind (_outactor _returnvalue_3) (`LevelSequencePlayer.CreateLevelSequencePlayer` (`|GetArrayItem` (`self.Sequences`) CoreIndex)))
      (`MovieSceneSequencePlayer.Play` _returnvalue_3)
      (`EnhancedInputSubsystemInterface.ClearAllMappings` (pcsubsystem `EnhancedInputLocalPlayerSubsystem` _returnvalue))
      (`KismetSystemLibrary.Delay` 10.0)
      (bind _returnvalue_4 (`|CreateWidget` "/Game/FrontierDestiny/98_Lose/WBP_Lose.WBP_Lose_C" _returnvalue))
      (`UserWidget.AddToViewport` _returnvalue_4 0)
      (bind _astower_demo_player_controller (cast `TowerDemoPlayerController` _returnvalue))
      (`TowerDemoPlayerController.FreeMouse` _astower_demo_player_controller _returnvalue_4)
      (`GameplayStatics.SetGamePaused` true))
    (:`then_1`
      (`GameplayStatics.PlaySound2D` "/Game/FrontierDestiny/98_Lose/Sounds/LoseSequence_Lose.LoseSequence_Lose" 2.0 1.0 0.0 null null))
    (:`then_2`
      (`|SpawnActorFromClass` "/Game/FrontierDestiny/98_Lose/BP_LoseExplosion.BP_LoseExplosion_C" (`self.GetTransform` _returnvalue_2) "AlwaysSpawn" "MultiplyWithRoot" null null))
    (:`then_3`
      (for _array_element (`self.GetAttachedActors` _returnvalue_2 true true)
        (`self.K2_SetActorLocation` _array_element (0.0 0.0 0.0) false false))
      (`self.K2_DestroyActor` _returnvalue_2))))

(fn `UserConstructionScript`)