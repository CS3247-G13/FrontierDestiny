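; Background music controller that switches between normal and horde music based on enemy wave state.
; On BeginPlay it binds to the EnemyWaveManager subsystem's horde begin and finished events and starts the normal BGM cue.
; When a horde begins it stops the normal cue and plays the horde cue, reversing this when the horde finishes.
; Switches are hard stop and play from the start, with no fades.
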(event `self.ReceiveBeginPlay`
  (bind _returnvalue (subsystem `EnemyWaveManagerSubsystem`))
  (add `EnemyWaveManagerSubsystem.OnHordeBegin` _returnvalue (delegate `Horde BGM Start`))
  (add `EnemyWaveManagerSubsystem.OnHordeFinished` _returnvalue (delegate `OnHordeFinished_Event`))
  (`AudioComponent.Play` (`self.Cue_BGM`) 0.0)
  (`AudioComponent.Stop` (`self.Cue_HordeBGM`)))

(event `Horde BGM Start`
  (params (HordeID :type Name))
  (`AudioComponent.Stop` (`self.Cue_BGM`))
  (`AudioComponent.Play` (`self.Cue_HordeBGM`) 0.0))

(event `OnHordeFinished_Event`
  (params (HordeID :type Name))
  (`AudioComponent.Stop` (`self.Cue_HordeBGM`))
  (`AudioComponent.Play` (`self.Cue_BGM`) 0.0))

(fn `UserConstructionScript`)