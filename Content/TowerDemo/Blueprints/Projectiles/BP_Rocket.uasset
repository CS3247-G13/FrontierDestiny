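; BP_Rocket is a rocket projectile in the tower demo that damages enemies it hits and expires after its Lifespan.
; HitTarget applies fixed damage to targets that cast to EnemyActor, crediting the rocket's instigator controller.
; For any target, it then prints the name and hit location as debug text and calls the parent HitTarget.
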(event `self.ReceiveBeginPlay`
  (`self.SetLifeSpan` (`self.Lifespan`)))

(event `self.HitTarget`
  (params (TargetActor :type "Actor Object Reference") (HitLocation :type "Vector Structure"))
  (`|ExecutionSequence`
    (:`then_0`
      (bind _asenemy_actor (cast `EnemyActor` TargetActor))
      (`GameplayStatics.ApplyDamage` _asenemy_actor 10.0 (`self.GetInstigatorController`) self))
    (:`then_1`
      (`KismetSystemLibrary.PrintString` (`KismetStringLibrary.Concat_StrStr` (`KismetSystemLibrary.GetDisplayName` TargetActor) ", " (`KismetStringLibrary.Conv_VectorToString` HitLocation)))
      (`parent.HitTarget` TargetActor HitLocation))))

(fn `UserConstructionScript`)