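; EnemyA is an enemy actor in TowerDemo that wanders between random points inside a bounding box, pausing at each one.
; Tick advances a clamped progress value scaled by distance for constant speed, then lerps the actor's location with sweep.
; On arrival, a DoOnce gates a timed pause before PickRandomLocation chooses the next point.
; BeginPlay's saved actor location is immediately overwritten by TargetLocation's initial value in PickRandomLocation.
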(event `self.ReceiveBeginPlay`
  (set `self.Previous Location` (`self.K2_GetActorLocation`))
  (`self.PickRandomLocation`))

(event `self.ReceiveTick`
  (params (DeltaSeconds :type "Float (single-precision)"))
  (if (not (`self.isPaused`))
    (`|ExecutionSequence`
      (:`then_0`
        ; Increment Progress
        (set `self.Progress` (`KismetMathLibrary.FClamp` (+ (`self.Progress`) (* (/ 1.0 (/ (`KismetMathLibrary.Vector_Distance` (`self.Previous Location`) (`self.Target Location`)) (`self.Speed`))) DeltaSeconds)))))
      (:`then_1`
        ; Set actor location
        (`self.K2_SetActorLocation` (`KismetMathLibrary.VLerp` (`self.Previous Location`) (`self.Target Location`) (`self.Progress`)) true))
      (:`then_2`
        ; If reached, pause
        (if (>= (`self.Progress`) 1.0)
          (`/Engine/EditorBlueprintResources/StandardMacros.DoOnce` false :!label _label
            (:`Completed`
              (set `self.isPaused` true)
              (`KismetSystemLibrary.Delay` (`self.Pause Duration`))
              (set `self.isPaused` false)
              (`self.PickRandomLocation`)
              (goto _label :!via `Reset`))))))))

(fn `PickRandomLocation`
  (set `self.Progress` 0.0)
  (set `self.Previous Location` (`self.Target Location`))
  (set `self.Target Location` (`KismetMathLibrary.RandomPointInBoundingBox` (`self.BoundingBoxCenter`) (`self.BoundingBoxHalfSize`))))

(fn `UserConstructionScript`)