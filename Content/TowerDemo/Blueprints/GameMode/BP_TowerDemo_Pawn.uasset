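; Player pawn for the TowerDemo game mode that turns Enhanced Input into camera look and planar movement.
; IA_Look drives controller yaw and pitch.
; IA_Move normalizes the 2D input and applies it along forward (X) and right (Y) vectors built from control yaw alone, so looking up or down does not tilt movement.
; Movement input is scaled by Speed and world delta time.
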(event `EnhancedInput|/Game/TowerDemo/Input/IA_Look`
  (params (ActionValue :type "Vector2D Structure") (ElapsedSeconds :type "Float (double-precision)") (TriggeredSeconds :type "Float (double-precision)") (InputAction :type "InputAction Object Reference" :default "/Game/TowerDemo/Input/IA_Look.IA_Look"))
  (bind (_x _y) (`KismetMathLibrary.BreakVector2D` ActionValue))
  ; Camera
  (:`Triggered`
    (`|ExecutionSequence`
      (:`then_0`
        (`self.AddControllerYawInput` _x))
      (:`then_1`
        (bind _result (`/Engine/EditorBlueprintResources/StandardMacros.NegateFloat` _y)
          (:`  `
            (`self.AddControllerPitchInput` _result)))))))

(event `EnhancedInput|/Game/TowerDemo/Input/IA_Move`
  (params (ActionValue :type "Vector2D Structure") (ElapsedSeconds :type "Float (double-precision)") (TriggeredSeconds :type "Float (double-precision)") (InputAction :type "InputAction Object Reference" :default "/Game/TowerDemo/Input/IA_Move.IA_Move"))
  (bind (_x _y) (`KismetMathLibrary.BreakVector2D` (`KismetMathLibrary.NormalSafe2D` ActionValue)))
  (bind _returnvalue (* (`GameplayStatics.GetWorldDeltaSeconds`) (`self.Speed`)))
  (bind _returnvalue_2 (`KismetMathLibrary.MakeRotator` 0.0 0.0 (.yaw (`self.GetControlRotation`))))
  ; Movement
  (:`Triggered`
    (`self.AddMovementInput` (* _x (`KismetMathLibrary.GetForwardVector` _returnvalue_2)) _returnvalue)
    (`self.AddMovementInput` (* _y (`KismetMathLibrary.GetRightVector` _returnvalue_2)) _returnvalue)))

(fn `UserConstructionScript`)