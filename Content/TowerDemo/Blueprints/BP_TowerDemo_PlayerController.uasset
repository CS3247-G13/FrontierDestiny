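; Player controller for the tower demo that adds the HUD and runs grid-based tower build mode, with hotbar selection and a debug enemy spawner.
; Each tick in build mode, a camera trace finds the grid cell, offsets it by the rotated tower pivot and checks placement.
; Rotation combines camera yaw snapped to 90 degrees with manual turns.
; A ghost tower follows, respawning when selection or validity changes; interact places the real tower.
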(event `self.ReceiveBeginPlay`
  ; Initialization, adds the HUD overlay and spawns the ghost structure
  (bind _returnvalue (`|CreateWidget` "/Game/TowerDemo/Blueprints/WBP_MainHUD.WBP_MainHUD_C" self))
  (`UserWidget.AddToPlayerScreen` _returnvalue 0))

(event `EnhancedInput|/Game/TowerDemo/Input/IA_Interact`
  (params (ActionValue :type Boolean) (ElapsedSeconds :type "Float (double-precision)") (TriggeredSeconds :type "Float (double-precision)") (InputAction :type "InputAction Object Reference" :default "/Game/TowerDemo/Input/IA_Interact.IA_Interact"))
  (bind _output (`self.GetSelectedTowerData`))
  ; Placing tower, triggered by left click
  (:`Started`
    (if (and (`self.InBuildMode`) (`self.CanBuild`))
      (bind _returnvalue (`|SpawnActorFromClass` (`TowerData.TowerBlueprint` _output) (`self.StructureTransform`) "Undefined" "MultiplyWithRoot" null false false self _output null))
      (`GridActor.PlaceTower` (`self.TargetGrid`) (`self.PivotPointGridIndex`) (`KismetMathLibrary.ComposeRotators` (`self.PlayerRotation`) (`self.BuildingRotation`)) _returnvalue))))

(event `self.ReceiveTick`
  (params (DeltaSeconds :type "Float (single-precision)"))
  (bind (_x _y) (break `IntPoint` (`TowerData.PivotPoint` (`self.GetSelectedTowerData`))))
  (bind _returnvalue (`KismetMathLibrary.MakeRotator` 0.0 0.0 (* (`KismetMathLibrary.Conv_IntToDouble` (`KismetMathLibrary.Round` (/ (.yaw (`.Rotation` (`self.GetPlayerViewPoint` self))) 90.0))) 90.0)))
  (bind _returnvalue_2 (`KismetMathLibrary.ComposeRotators` (`self.BuildingRotation`) _returnvalue))
  ; Every frame, the ghost structure is moved
  (if (`self.InBuildMode`)
    (bind (_grid _outsnappedlocation) (`self.RaycastToGrid`))
    (`|ExecutionSequence`
      (:`then_0`
        (set `self.PlayerRotation` _returnvalue))
      (:`then_1`
        (bind _returnvalue_3 (+ _outsnappedlocation (`KismetMathLibrary.Conv_Vector2DToIntPoint` (`KismetMathLibrary.Conv_VectorToVector2D` (`KismetMathLibrary.GreaterGreater_VectorRotator` (`KismetMathLibrary.NegateVector` (`KismetMathLibrary.MakeVector` (`KismetMathLibrary.Conv_IntToDouble` _x) (`KismetMathLibrary.Conv_IntToDouble` _y))) _returnvalue_2)))))
        (set `self.PivotPointGridIndex` _returnvalue_3))
      (:`then_2`
        (set `self.TargetGrid` _grid))
      (:`then_3`
        (bind _returnvalue_4 (`GridActor.CanPlaceTower` _grid _returnvalue_3 _returnvalue_2 (`self.GetSelectedTowerData`)))
        (`|ExecutionSequence`
          (:`then_0`
            (if (xor _returnvalue_4 (`self.CanBuild`))
              (`/Engine/EditorBlueprintResources/StandardMacros.DoOnce` false :!via `Reset`
                (:`Completed`
                  (`self.UpdateGhostStructureModel`)))))
          (:`then_1`
            (set `self.CanBuild` _returnvalue_4)
            (bind _output_get (set `self.StructureTransform` (`KismetMathLibrary.MakeTransform` (`GridActor.GetWorldLocationFromGridIndex` _grid _returnvalue_3 _returnvalue_2) _returnvalue_2)))
            (`self.UpdateGhostStructureModel`)
            (`self.K2_SetActorTransform` (`self.GhostStructure`) _output_get false true)))))))

(event `EnhancedInput|/Game/TowerDemo/Input/IA_Rotate`
  (params (ActionValue :type "Float (double-precision)") (ElapsedSeconds :type "Float (double-precision)") (TriggeredSeconds :type "Float (double-precision)") (InputAction :type "InputAction Object Reference" :default "/Game/TowerDemo/Input/IA_Rotate.IA_Rotate"))
  ; Rotate on input (On top of rotate w.r.t camera)
  (:`Started`
    (set `self.BuildingRotation` (`KismetMathLibrary.ComposeRotators` (`self.BuildingRotation`) (`KismetMathLibrary.MakeRotator` 0.0 0.0 (* 90.0 ActionValue))))))

(event `EnhancedInput|/Game/TowerDemo/Input/IA_Debug`
  (params (ActionValue :type Boolean) (ElapsedSeconds :type "Float (double-precision)") (TriggeredSeconds :type "Float (double-precision)") (InputAction :type "InputAction Object Reference" :default "/Game/TowerDemo/Input/IA_Debug.IA_Debug"))
  ; Spawn enemies
  (:`Triggered`
    (bind _returnvalue (`|SpawnActorFromClass` "/Game/TowerDemo/Blueprints/EnemyA.EnemyA_C" (`self.GetTransform` (`self.K2_GetPawn`)) "Undefined" "MultiplyWithRoot" null null))
    (`|ExecutionSequence`
      (:`then_0`
        (set `EnemyActor.MaxHealth` 1000 _returnvalue)
        (set `EnemyActor.CurrentHealth` 1000 _returnvalue))
      (:`then_1`
        (set `/Game/TowerDemo/Blueprints/EnemyA.BoundingBoxCenter` (`self.K2_GetActorLocation` (`self.K2_GetPawn`)) _returnvalue)
        (set `/Game/TowerDemo/Blueprints/EnemyA.BoundingBoxHalfSize` (650.0 650.0 0.0) _returnvalue))
      (:`then_2`
        (set `/Game/TowerDemo/Blueprints/EnemyA.Speed` (`KismetMathLibrary.RandomFloatInRange` 100.0 500.0) _returnvalue)
        (set `/Game/TowerDemo/Blueprints/EnemyA.Pause Duration` (`KismetMathLibrary.RandomFloatInRange` 0.0 3.0) _returnvalue)
        (`/Game/TowerDemo/Blueprints/EnemyA.PickRandomLocation` _returnvalue)))))

(event `EnhancedInput|/Game/TowerDemo/Input/IA_SelectSlot`
  (params (ActionValue :type "Float (double-precision)") (ElapsedSeconds :type "Float (double-precision)") (TriggeredSeconds :type "Float (double-precision)") (InputAction :type "InputAction Object Reference" :default "/Game/TowerDemo/Input/IA_SelectSlot.IA_SelectSlot"))
  (bind _returnvalue (`KismetArrayLibrary.Array_Length` (`self.AvailableTowerData`)))
  (bind _returnvalue_2 (`KismetMathLibrary.FTrunc` (- ActionValue 1.0)))
  ; When a hotbar number is pressed, the tower is selected and enters build mode if not already in
  (:`Started`
    (if (>= _returnvalue_2 _returnvalue)
      (`KismetSystemLibrary.RaiseScriptError` (`KismetStringLibrary.Concat_StrStr` "Tower index out of bounds. Max " (`KismetStringLibrary.Conv_IntToString` (- _returnvalue 1)) ", received " (`KismetStringLibrary.Conv_IntToString` _returnvalue_2)))
      (else
        (`|ExecutionSequence`
          (:`then_0`
            (if (not (`self.InBuildMode`))
              (`self.EnterBuildMode`)))
          (:`then_1`
            (`self.UpdateSelectedTower` _returnvalue_2)))))))

(event `EnhancedInput|/Game/TowerDemo/Input/IA_ToggleBuildMode`
  (params (ActionValue :type Boolean) (ElapsedSeconds :type "Float (double-precision)") (TriggeredSeconds :type "Float (double-precision)") (InputAction :type "InputAction Object Reference" :default "/Game/TowerDemo/Input/IA_ToggleBuildMode.IA_ToggleBuildMode"))
  ; Press V to toggle build mode
  (:`Started`
    (if (`self.InBuildMode`)
      (`self.ExitBuildMode`)
      (else
        (`self.EnterBuildMode`)))))

(fn `EnterBuildMode`
  (set `self.InBuildMode` true)
  (if (== (`self.SelectedTower`) -1)
    _))

(fn `ExitBuildMode`
  (set `self.InBuildMode` false)
  (`self.HideGhostStructure`))

(fn `UpdateSelectedTower`
  (params (Tower :type Integer))
  (`KismetSystemLibrary.PrintString` "Calling update selected tower")
  (set `self.SelectedTower` Tower)
  (if (`self.InBuildMode`)
    (`self.UpdateGhostStructureModel`)))

(fn `UserConstructionScript`)