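; Player pawn for the TowerDemo that provides look and planar movement through Enhanced Input.
; It adds its mapping context on BeginPlay and feeds look input into controller yaw and pitch.
; Move input is normalized, scaled by speed and frame delta time, then applied as a swept local XY offset, without using a movement component.
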(event `self.ReceiveBeginPlay`
  ; Add Mapping Context
  (`EnhancedInputSubsystemInterface.AddMappingContext` (subsystem `EnhancedInputLocalPlayerSubsystem`) "/Game/TowerDemo/Input/IMC_TowerDemo.IMC_TowerDemo" 0 (struct)))

(event `EnhancedInput|/Game/TowerDemo/Input/IA_Look`
  (params (ActionValue :type "Vector2D Structure") (ElapsedSeconds :type "Float (double-precision)") (TriggeredSeconds :type "Float (double-precision)") (InputAction :type "InputAction Object Reference" :default "/Game/TowerDemo/Input/IA_Look.IA_Look"))
  (bind (_x _y) (`KismetMathLibrary.BreakVector2D` ActionValue))
  ; Camera
  (:`Triggered`
    (`|ExecutionSequence`
      (:`then_0`
        (`self.AddControllerYawInput` _x))
      (:`then_1`
        (bind _result (`/Engine/EditorBlueprintResources/StandardMacros.NegateFloat` _y)
          (:`  `
            (`self.AddControllerPitchInput` _result)))))))

(event `EnhancedInput|/Game/TowerDemo/Input/IA_Move`
  (params (ActionValue :type "Vector2D Structure") (ElapsedSeconds :type "Float (double-precision)") (TriggeredSeconds :type "Float (double-precision)") (InputAction :type "InputAction Object Reference" :default "/Game/TowerDemo/Input/IA_Move.IA_Move"))
  ; Movement
  (:`Triggered`
    (`self.K2_AddActorLocalOffset` (`KismetMathLibrary.Conv_Vector2DToVector` (* (* (`GameplayStatics.GetWorldDeltaSeconds`) (`self.Speed`)) (`KismetMathLibrary.NormalSafe2D` ActionValue 0.001))) true)))

(fn `UserConstructionScript`)