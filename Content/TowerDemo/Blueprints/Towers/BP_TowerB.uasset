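; BP_TowerB is a twin-gun tower that fires homing rockets at its current target.
; Each tick, the head turns at constant speed, on yaw only, toward the target's "Target"-tagged component.
; When the Cooldown component finishes and a target exists, it spawns a BP_Rocket from the left gun, restarts the cooldown, then fires the right gun after a short delay.
; Rockets receive launch velocity, target, turn speed and departure clearance duration at spawn.
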(event `self.ReceiveBeginPlay`
  (`CooldownComponent.StartCooldown` (`self.Cooldown`)))

(event `self.ReceiveTick`
  (params (DeltaSeconds :type "Float (single-precision)"))
  (bind _towerb_head (`self.TowerB_Head`))
  (if (not (`self.TargetIsNull`))
    (`SceneComponent.K2_SetWorldRotation` (`self.TowerB_Head`) (`KismetMathLibrary.RInterpTo_Constant` (`self.IsolateYaw` (`SceneComponent.K2_GetComponentRotation` _towerb_head)) (`self.IsolateYaw` (`KismetMathLibrary.MakeRotFromX` (`KismetMathLibrary.GetDirectionUnitVector` (`SceneComponent.K2_GetComponentLocation` _towerb_head) (`SceneComponent.K2_GetComponentLocation` (`|GetArrayItem` (`self.GetComponentsByTag` (`self.CurrentTarget`) "/Script/Engine.SceneComponent" "Target")))))) DeltaSeconds (`self.HeadRotationSpeed`)) false false)))

(event `self.Cooldown.OnCooldownFinished`
  (bind _cooldown (`self.Cooldown`))
  (bind _success (`self.TryAttackTarget` (`SceneComponent.K2_GetComponentToWorld` (`self.LeftGun`)) (`SceneComponent.GetForwardVector` (`self.TowerB_Head`))))
  (if _success
    (`CooldownComponent.ResetCooldown` _cooldown)
    (`CooldownComponent.StartCooldown` _cooldown)
    (`KismetSystemLibrary.Delay` 0.2)
    (`self.TryAttackTarget` (`SceneComponent.K2_GetComponentToWorld` (`self.RightGun`)) (`SceneComponent.GetForwardVector` (`self.TowerB_Head`)))))

(fn `TryAttackTarget`
  (params (`Spawn Location` :type "Transform Structure") (`Forward Vector` :type "Vector Structure"))
  (returns (Success :type Boolean))
  (if (`self.TargetIsNull`)
    (return false)
    (else
      (`|SpawnActorFromClass` "/Game/TowerDemo/Blueprints/Projectiles/BP_Rocket.BP_Rocket_C" `Spawn Location` "AlwaysSpawn" "OverrideRootScale" self 30.0 (* `Forward Vector` (`self.RocketTravelSpeed`)) (`|GetArrayItem` (`self.GetComponentsByTag` (`self.CurrentTarget`) "/Script/Engine.SceneComponent" "Target")) (`self.RocketRotationalSpeed`) (`self.RocketDepartureDuration`) (`self.GetInstigator`))
      (return true))))

(fn `UserConstructionScript`)