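; Base Blueprint for single-target towers in a tower demo, which pick an enemy inside their range and attack it on a cooldown.
; Looping timers refresh overlapping enemies and reselect the target, alongside overlap events on a range volume scaled from Range.
; Tick counts down the cooldown and drives rotation and attack through stub functions, presumably for child overrides.
; Ghost instances instead disable ticking and show valid or invalid placement materials.
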(event `self.ReceiveBeginPlay`
  (bind _returnvalue (+ (`self.Range`) 1.0))
  (if (`self.bIsGhost`)
    ; Ghost structure
    (`self.SetActorTickEnabled` false)
    (for _array_element (`self.K2_GetComponentsByClass` "/Script/Engine.PrimitiveComponent")
      (for _index (range (`PrimitiveComponent.GetNumMaterials` _array_element))
        (`PrimitiveComponent.SetMaterial` _array_element _index (select `bool` (`self.bIsValidGhost`) :`false` "/Game/TowerDemo/Materials/M_TowerGhost_Invalid.M_TowerGhost_Invalid" :`true` "/Game/TowerDemo/Materials/M_TowerGhost.M_TowerGhost" :!type "Material Object Reference"))))
    (else
      (`self.UpdatePotentialEnemies`)
      (`self.SelectTargetEnemy`)
      (`KismetSystemLibrary.K2_SetTimer` null "UpdatePotentialEnemies" 0.5 true)
      (`KismetSystemLibrary.K2_SetTimer` null "SelectTargetEnemy" 0.1 true)
      (`SceneComponent.SetRelativeScale3D` (`self.RangeDetection`) (`KismetMathLibrary.MakeVector` _returnvalue _returnvalue _returnvalue)))))

(event `self.ReceiveTick`
  (params (DeltaSeconds :type "Float (single-precision)"))
  (`|ExecutionSequence`
    (:`then_0`
      ; Tick the cooldown
      (set `self.CurrentCooldown` (`KismetMathLibrary.FClamp` (- (`self.CurrentCooldown`) DeltaSeconds) 0.0 (`self.Cooldown`))))
    (:`then_1`
      (if (!= (`self.Target`) null)
        (`|ExecutionSequence`
          (:`then_0`
            (`self.RotateToFaceEnemy` DeltaSeconds))
          (:`then_1`
            ; Attack
            (bind _can_attack_enemy (`self.CanAttackEnemy`))
            (if _can_attack_enemy
              (if (== (`self.CurrentCooldown`) 0.0)
                (bind _success (`self.AttackNearestEnemy`))
                (if _success
                  (`self.ResetCooldown`))))))))))

(event `self.RangeDetection.OnComponentBeginOverlap`
  (params (OverlappedComponent :type "PrimitiveComponent Object Reference") (OtherActor :type "Actor Object Reference") (OtherComp :type "PrimitiveComponent Object Reference") (OtherBodyIndex :type Integer) (bFromSweep :type Boolean) (SweepResult :type "HitResult Structure (by ref)"))
  (bind _asenemy_actor (cast `EnemyActor` OtherActor))
  (`KismetArrayLibrary.Array_Add` (`self.PotentialTargets`) _asenemy_actor))

(event `self.RangeDetection.OnComponentEndOverlap`
  (params (OverlappedComponent :type "PrimitiveComponent Object Reference") (OtherActor :type "Actor Object Reference") (OtherComp :type "PrimitiveComponent Object Reference") (OtherBodyIndex :type Integer))
  (bind _asenemy_actor (cast `EnemyActor` OtherActor))
  (`KismetArrayLibrary.Array_RemoveItem` (`self.PotentialTargets`) _asenemy_actor))

(fn `AttackNearestEnemy`
  (returns (success :type Boolean)))

(fn `CanAttackEnemy`
  (returns (`Can Attack Enemy` :type Boolean))
  (return false))

(fn `ResetCooldown`
  (set `self.CurrentCooldown` (`self.Cooldown`)))

(fn `RotateToFaceEnemy`
  (params (DeltaTime :type "Float (double-precision)")))

(fn `SelectTargetEnemy`
  (`self.SelectTarget`))

(fn `UpdatePotentialEnemies`
  (bind _output_get (set `self.PotentialTargets` (`self.GetOverlappingActors` "/Script/FrontierDestiny.EnemyActor")))
  (if (not (`KismetArrayLibrary.Array_Contains` _output_get (`self.Target`)))
    (`self.SelectTarget`)))

(fn `UserConstructionScript`
  (if (`self.bIsGhost`)
    _))