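; TowerB is a tower that attacks its target with a two-shot laser burst from a rotating head.
; Its head turns toward the target at constant speed on yaw only, using a negated direction vector, and can attack once horizontal alignment passes a dot-product threshold.
; Each attack fires immediately and again after a short timer, with each successful hit attempt playing the laser sound from its own sound source.
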(fn `AttackNearestEnemy`
  (returns (success :type Boolean))
  (`self.PerformAttack` (`SceneComponent.K2_GetComponentLocation` (`self.SoundSource1`)))
  (`KismetSystemLibrary.K2_SetTimer` null "PerformSecondAttack" 0.2)
  (return true))

(fn `CanAttackEnemy`
  (returns (`Can Attack Enemy` :type Boolean))
  (return (> (`KismetMathLibrary.Dot_VectorVector` (`KismetMathLibrary.Normal` (`self.IsolateXY` (`SceneComponent.GetForwardVector` (`self.TowerB_Head`)))) (`KismetMathLibrary.Normal` (`self.IsolateXY` (`self.GetUnitDirectionToTarget`)))) 0.9)))

(fn `PerformAttack`
  (params (`Sound Location` :type "Vector Structure"))
  (bind _returnvalue (`self.AttackTarget`))
  (if _returnvalue
    (`GameplayStatics.PlaySoundAtLocation` "/Game/TowerDemo/Sounds/SW_Laser.SW_Laser" `Sound Location` (struct) 1.0 1.0 0.0 null null null null)))

(fn `PerformSecondAttack`
  (`self.PerformAttack` (`SceneComponent.K2_GetComponentLocation` (`self.SoundSource2`))))

(fn `RotateToFaceEnemy`
  (params (DeltaTime :type "Float (double-precision)"))
  (bind _towerb_head (`self.TowerB_Head`))
  (`SceneComponent.K2_SetWorldRotation` (`self.TowerB_Head`) (`KismetMathLibrary.RInterpTo_Constant` (`self.IsolateYaw` (`SceneComponent.K2_GetComponentRotation` _towerb_head)) (`self.IsolateYaw` (`KismetMathLibrary.Conv_VectorToRotator` (`KismetMathLibrary.NegateVector` (`KismetMathLibrary.GetDirectionUnitVector` (`SceneComponent.K2_GetComponentLocation` _towerb_head) (`self.K2_GetActorLocation` (`self.Target`)))))) DeltaTime (`self.RotationSpeed`)) false false))

(fn `UserConstructionScript`
  (`parent.UserConstructionScript`))