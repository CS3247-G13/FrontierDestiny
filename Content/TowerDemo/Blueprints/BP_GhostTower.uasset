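; BP_GhostTower is a translucent-style stand-in actor for a tower, showing a given mesh in the M_TowerGhost material.
; It starts hidden with actor tick disabled, and SetVisible toggles the Model component's visibility without propagating to children.
; UpdateModel swaps Model's static mesh, then overrides every material slot with the ghost material, so any supplied mesh gets the same look.
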(event `self.ReceiveBeginPlay`
  (`self.SetActorTickEnabled` false)
  (`self.SetVisible` false))

(fn `SetVisible`
  (params (Visible :type Boolean))
  (`SceneComponent.SetVisibility` (`self.Model`) Visible false))

(fn `UpdateModel`
  (params (Mesh :type "StaticMesh Object Reference"))
  (bind _model (`self.Model`))
  (`StaticMeshComponent.SetStaticMesh` (`self.Model`) Mesh)
  (for _index (range (`PrimitiveComponent.GetNumMaterials` _model))
    (`PrimitiveComponent.SetMaterial` _model _index "/Game/TowerDemo/Materials/M_TowerGhost.M_TowerGhost")))

(fn `UserConstructionScript`)